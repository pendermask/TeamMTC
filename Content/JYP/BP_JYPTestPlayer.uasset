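; BP_JYPTestPlayer is a first-person test player that can look at a D4 die and roll it.
; Each tick it line-traces 1000 units forward from the camera against tracked object types, storing a hit BP_D4 and setting a flag, which clears when nothing is hit.
; Pressing E while the flag is set calls Rolling on the stored die.
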(event `self.ReceiveTick`
  (params (DeltaSeconds :type "Float (single-precision)"))
  (bind _firstpersoncameracomponent (`self.FirstPersonCameraComponent`))
  (bind _returnvalue (`SceneComponent.K2_GetComponentLocation` _firstpersoncameracomponent))
  (bind (_outhit _returnvalue_2) (`KismetSystemLibrary.LineTraceSingleForObjects` _returnvalue (+ (* (`SceneComponent.GetForwardVector` _firstpersoncameracomponent) 1000.0) _returnvalue) (`self.PlayerTrackingObjectTypes`)))
  (if _returnvalue_2
    (bind _asbp_d4 (cast `/Game/JYP/BP_D4` (`.HitActor` (`GameplayStatics.BreakHitResult` _outhit))))
    (set `self.bDiceHere?` true)
    (set `self.dice` _asbp_d4)
    (else
      (set `self.bDiceHere?` false))))

(event `Key|E`
  (params (Key :type "Key Structure"))
  (:`Pressed`
    (if (`self.bDiceHere?`)
      (`/Game/JYP/BP_D4.Rolling` (`self.dice`)))))

(fn `UserConstructionScript`)