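; First-person test player for a turn-based tower game, handling aiming, interaction, floor progression and monster actions.
; A per-tick forward sphere trace outlines highlightable actors and tracks whether a letter or monster is in view.
; Right-click opens the letter or starts Magician dialogue, and E loads the next floor by current level name.
; Number keys spend the turn on death, life, grace or normal actions, tallied in the GameInstance.
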(event `Key|LeftMouseButton`
  (params (Key :type "Key Structure"))
  ;[1 1 1] Not use
)

(event `Key|E`
  (params (Key :type "Key Structure"))
  (:`Pressed`
    (if (`self.bPlayerCanPressNextDoor?`)
      (bind _returnvalue (`GameplayStatics.GetCurrentLevelName` true))
      (`|ExecutionSequence`
        (:`then_0`
          (if (`KismetStringLibrary.EqualEqual_StrStr` _returnvalue "JYPOpening")
            (if (`self.bLetterTextHere?`)
              (`GameplayStatics.OpenLevel` "JYPTowerLobbyFloor_Lobby"))))
        (:`then_1`
          (if (`KismetStringLibrary.EqualEqual_StrStr` _returnvalue "JYPTowerLobbyFloor_Lobby")
            (`GameplayStatics.OpenLevel` "JYPTowerFirstFloor_Normal")))
        (:`then_2`
          (if (`KismetStringLibrary.EqualEqual_StrStr` _returnvalue "JYPTowerFirstFloor_Normal")
            (`GameplayStatics.OpenLevel` "JYPTowerSecondFloor_Grace")))
        (:`then_3`
          (if (`KismetStringLibrary.EqualEqual_StrStr` _returnvalue "JYPTowerSecondFloor_Grace")
            (`GameplayStatics.OpenLevel` "JYPTowerThirdFloor_Life")))
        (:`then_4`
          (if (`KismetStringLibrary.EqualEqual_StrStr` _returnvalue "JYPTowerThirdFloor_Life")
            (`GameplayStatics.OpenLevel` "JYPTowerFourthFloor_Death")))
        (:`then_5`
          (if (`KismetStringLibrary.EqualEqual_StrStr` _returnvalue "JYPTowerFourthFloor_Death")
            (`GameplayStatics.OpenLevel` "JYPTowerLastFloor_Magician")))
        (:`then_6`
          (if (`KismetStringLibrary.EqualEqual_StrStr` _returnvalue "JYPTowerLastFloor_Magician")
            (bind _returnvalue_2 (`GameplayStatics.GetActorOfClass` "/Game/JYP/Blueprints/BP_Restart.BP_Restart_C"))
            (`/Game/JYP/Blueprints/BP_Restart.Restart` _returnvalue_2)
            (`GameplayStatics.OpenLevel` "JYPTowerLobbyFloor_Lobby")))))))

(event `self.ReceiveTick`
  (params (DeltaSeconds :type "Float (single-precision)"))
  (bind _firstpersoncameracomponent (`self.FirstPersonCameraComponent`))
  (bind _returnvalue (`SceneComponent.K2_GetComponentLocation` _firstpersoncameracomponent))
  (bind (_outhit _returnvalue_2) (`KismetSystemLibrary.SphereTraceSingleForObjects` :`Start` _returnvalue :`End` (+ (* (`SceneComponent.GetForwardVector` _firstpersoncameracomponent) 1000.0) _returnvalue) :`Radius` 15.0 :`ObjectTypes` (`self.PlayerTrackingObjectTypes`) :`DrawDebugType` "ForOneFrame"))
  (if _returnvalue_2
    (`|ExecutionSequence`
      (:`then_0`
        (bind (_bblockinghit _binitialoverlap _time _distance _location _impactpoint _normal _impactnormal _physmat _hitactor) (`GameplayStatics.BreakHitResult` _outhit))
        (bind _returnvalue_3 (`self.GetComponentByClass` _hitactor "/Game/JYP/Blueprints/BP_HighlightComp.BP_HighlightComp_C"))
        (`/Engine/EditorBlueprintResources/StandardMacros.IsValid` _returnvalue_3
          (:`Is Valid`
            (`/Game/JYP/Blueprints/BP_HighlightComp.OnOutline` _returnvalue_3))))
      (:`then_1`
        (bind _asbp_letter (cast `/Game/JYP/Blueprints/BP_Letter` _hitactor))
        (set `self.bLetterHere?` true)
        (set `self.Letter` _asbp_letter))
      (:`then_2`
        (cast `/Game/JYP/Blueprints/Monster/BP_MonsterParent` _hitactor
          (:`then`
            (set `self.bPlayerSeeMonster?` true))
          (:`CastFailed`
            (set `self.bPlayerSeeMonster?` false)))))
    (else
      (set `self.bLetterHere?` false))))

(event `self.ReceiveBeginPlay`
  ;[1 1 1] Cache
  (bind _asgi_game_instance (cast `/Game/JYP/Blueprints/GI_GameInstance` (`GameplayStatics.GetGameInstance`)))
  (set `self.GameInstance` _asgi_game_instance)
  (bind _asbp_jypgmb (cast `/Game/JYP/Blueprints/BP_JYPGMB` (`GameplayStatics.GetGameMode`)))
  (set `self.JYPGMB` _asbp_jypgmb))

(event `Key|RightMouseButton`
  (params (Key :type "Key Structure"))
  (bind _letter (`self.Letter`))
  ;[1 1 1] Comment
  (:`Pressed`
    (bind _returnvalue (`GameplayStatics.GetCurrentLevelName` true))
    (if (`KismetStringLibrary.EqualEqual_StrStr` _returnvalue "JYPOpening")
      (if (`self.bLetterHere?`)
        (if (`/Game/JYP/Blueprints/BP_Letter.bInteract?` _letter)
          (`/Game/JYP/Blueprints/BP_Letter.WhenClickLetter` _letter)
          (set `self.bLetterTextHere?` true))
        (else
          (`KismetSystemLibrary.PrintString` "retry!")))
      (elif (`KismetStringLibrary.EqualEqual_StrStr` _returnvalue "JYPTowerLastFloor_Magician")
        (bind _returnvalue_2 (`GameplayStatics.GetActorOfClass` "/Game/JYP/Blueprints/Monster/BP_Magician.BP_Magician_C"))
        (`/Game/JYP/Blueprints/Monster/BP_Magician.startDialogue` _returnvalue_2)))))

(event `Key|One`
  (params (Key :type "Key Structure"))
  (bind _healthcomp (`self.HealthComp`))
  (bind _gameinstance (`self.GameInstance`))
  ;[1 1 1] Comment
  ;;[1 1 1] death
  (:`Pressed`
    (`/Engine/EditorBlueprintResources/StandardMacros.IsValid` _healthcomp
      (:`Is Valid`
        (if (`self.bPlayerSeeMonster?`)
          (if (`/Game/JYP/Blueprints/BP_HealthComp.bAmIDie?` _healthcomp)
            _
            (elif (`self.bPlayerTurn?`)
              (`/Game/JYP/Blueprints/BP_HealthComp.Damaged` (`self.HealthComp`) (`self.damage`))
              (bind _output_get (set `/Game/JYP/Blueprints/GI_GameInstance.deathValue` (+ (`/Game/JYP/Blueprints/GI_GameInstance.deathValue` _gameinstance) (`self.damage`)) _gameinstance))
              (`KismetSystemLibrary.PrintString` (`KismetStringLibrary.Concat_StrStr` "current death value is " (`KismetStringLibrary.Conv_IntToString` _output_get)))
              (set `self.bPlayerTurn?` false)))
          (else
            (`KismetSystemLibrary.PrintString` "No Enemy Interaction.")))))))

(event `Key|Two`
  (params (Key :type "Key Structure"))
  (bind _gameinstance (`self.GameInstance`))
  ;[1 1 1] Comment
  ;;[1 1 1] life
  (:`Pressed`
    (if (`self.bPlayerSeeMonster?`)
      (if (`self.bPlayerTurn?`)
        (`/Game/JYP/Blueprints/BP_HealthComp.Healing` (`self.BP_HealthComp`) (`self.heal`))
        (bind _output_get (set `/Game/JYP/Blueprints/GI_GameInstance.lifeValue` (+ (`/Game/JYP/Blueprints/GI_GameInstance.lifeValue` _gameinstance) (`self.heal`)) _gameinstance))
        (`KismetSystemLibrary.PrintString` (`KismetStringLibrary.Concat_StrStr` "current life value is " (`KismetStringLibrary.Conv_IntToString` _output_get)))
        (set `self.bPlayerTurn?` false)))))

(event `Key|Three`
  (params (Key :type "Key Structure"))
  (bind _gameinstance (`self.GameInstance`))
  ;[1 1 1] Comment
  ;;[1 1 1] grace
  (:`Pressed`
    (if (`self.bPlayerSeeMonster?`)
      (if (`self.bPlayerTurn?`)
        (`/Game/JYP/Blueprints/BP_FriendshipComp.GetFriendship` (`self.FriendshipComp`) (`self.friendship`))
        (bind _output_get (set `/Game/JYP/Blueprints/GI_GameInstance.graceValue` (+ (`/Game/JYP/Blueprints/GI_GameInstance.graceValue` _gameinstance) (`self.friendship`)) _gameinstance))
        (`KismetSystemLibrary.PrintString` (`KismetStringLibrary.Concat_StrStr` "current grace value is" (`KismetStringLibrary.Conv_IntToString` _output_get)))
        (set `self.bPlayerTurn?` false)))))

(event `Key|Four`
  (params (Key :type "Key Structure"))
  (bind _gameinstance (`self.GameInstance`))
  ;[1 1 1] Comment
  ;;[1 1 1] normal
  (:`Pressed`
    (if (`self.bPlayerSeeMonster?`)
      (if (`self.bPlayerTurn?`)
        (bind _output_get (set `/Game/JYP/Blueprints/GI_GameInstance.normalValue` (+ (`/Game/JYP/Blueprints/GI_GameInstance.normalValue` _gameinstance) (`self.normal`)) _gameinstance))
        (`KismetSystemLibrary.PrintString` (`KismetStringLibrary.Concat_StrStr` "current normal value is " (`KismetStringLibrary.Conv_IntToString` _output_get)))
        (set `self.bPlayerTurn?` false)))))

(event `Key|Five`
  (params (Key :type "Key Structure"))
  ;[1 1 1] joker -  esca[e
)

(fn `UserConstructionScript`)