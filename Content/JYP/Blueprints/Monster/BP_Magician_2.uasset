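; Magician monster Blueprint that shows dialogue lines commenting on the player's run.
; On BeginPlay it caches the game instance, starts dialogue, then builds lines from monster kills, most-used card attribute, action count and total friendship.
; The attribute line comes from a name-to-count map searched for its maximum value.
; StartDialogue advances an index and shows that map entry on a TextRender, printing a debug string when none exists.
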(event `self.ReceiveBeginPlay`
  (bind _comparetypevalue (`self.compareTypeValue`))
  (bind _comparetypevalue_2 (`self.compareTypeValue`))
  (bind _gameinstance (`self.GameInstance`))
  (bind _dialogue (`self.dialogue`))
  (`|ExecutionSequence`
    (:`then_0`
      ;[1 1 1] Caching
      (bind _asgi_game_instance (cast `/Game/JYP/Blueprints/GI_GameInstance` (`GameplayStatics.GetGameInstance`)))
      (set `self.GameInstance` _asgi_game_instance)
      (`self.startDialogue`))
    (:`then_1`
      (`BlueprintMapLibrary.Map_Add` _comparetypevalue_2 "Normal" (`/Game/JYP/Blueprints/GI_GameInstance.normalValue` _gameinstance))
      (`BlueprintMapLibrary.Map_Add` _comparetypevalue_2 "Grace" (`/Game/JYP/Blueprints/GI_GameInstance.graceValue` _gameinstance))
      (`BlueprintMapLibrary.Map_Add` _comparetypevalue_2 "Life" (`/Game/JYP/Blueprints/GI_GameInstance.lifeValue` _gameinstance))
      (`BlueprintMapLibrary.Map_Add` _comparetypevalue_2 "Death" (`/Game/JYP/Blueprints/GI_GameInstance.deathValue` _gameinstance)))
    (:`then_2`
      ;[1 1 1] Set dialogue map
      (`BlueprintMapLibrary.Map_Add` _dialogue 5 (`KismetStringLibrary.Concat_StrStr` "You sacrificed " (`KismetStringLibrary.Conv_IntToString` (`/Game/JYP/Blueprints/GI_GameInstance.deadMonsterCount` (`self.GameInstance`))) " monsters to get up here."))
      (bind _values (`BlueprintMapLibrary.Map_Values` _comparetypevalue))
      (bind _keys (`BlueprintMapLibrary.Map_Keys` _comparetypevalue))
      (`BlueprintMapLibrary.Map_Add` _dialogue 7 (`KismetStringLibrary.Concat_StrStr` "You used the " (`|GetArrayItem` _keys (`KismetMathLibrary.MaxOfIntArray` _values)) " attribute card the most until you came up here..."))
      (`BlueprintMapLibrary.Map_Add` _dialogue 9 (`KismetStringLibrary.Concat_StrStr` "You've come this far with " (`KismetStringLibrary.Conv_IntToString` (`/Game/JYP/Blueprints/GI_GameInstance.playerActionCount` (`self.GameInstance`))) " choices."))
      (if (< (`/Game/JYP/Blueprints/GI_GameInstance.totalFriendship` (`self.GameInstance`)) 5)
        (`BlueprintMapLibrary.Map_Add` _dialogue 6 "You're quite liked by the monsters.")
        (else
          (`BlueprintMapLibrary.Map_Add` _dialogue 6 "Well, you're emotionally dry."))))))

(event `startDialogue`
  (bind (_value _returnvalue) (`BlueprintMapLibrary.Map_Find` (`self.dialogue`) (`self.dialogueIndex`)))
  ;[1 1 1] Dialogue
  (set `self.dialogueIndex` (+ (`self.dialogueIndex`) 1))
  (if _returnvalue
    (`TextRenderComponent.K2_SetText` (`self.TextRender`) (`KismetTextLibrary.Conv_StringToText` _value))
    (else
      (`KismetSystemLibrary.PrintString` "WWWWWWWWWWWWWWWWWWWWWWWWWWWW"))))

(fn `UserConstructionScript`)