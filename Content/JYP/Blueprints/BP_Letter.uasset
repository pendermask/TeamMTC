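; BP_Letter is an interactable letter that fades in at BeginPlay and can be clicked to reveal a child actor.
; The LetterAppearance timeline drives the Opacity material parameter on the Letterz component, enabling interaction and BPHighlightComp only when it finishes.
; WhenClickLetter, if interaction is enabled, hides Letterz, disables interaction and highlighting, and makes the ChildActor component visible.
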(event `self.ReceiveBeginPlay`
  ;[0 0 0 0 25] BeginPlay for Init
  (set `self.bInteract?` false)
  (set `/Game/JYP/Blueprints/BP_HighlightComp.bInteractable?` false (`self.BP_HighlightComp`))
  (`self.InitLetterAppearance`))

(event `InitLetterAppearance`
  ;[0 0 0 0 25] Dice Appearance
  (bind (_direction _diceupdate) (`Timeline|LetterAppearance` :!via `PlayFromStart`)
    (:`Update`
      (`MeshComponent.SetScalarParameterValueOnMaterials` (`self.Letterz`) "Opacity" _diceupdate))
    (:`Finished`
      (set `/Game/JYP/Blueprints/BP_HighlightComp.bInteractable?` true (`self.BP_HighlightComp`))
      (set `self.bInteract?` true))))

(event `WhenClickLetter`
  (if (`self.bInteract?`)
    (`SceneComponent.SetVisibility` (`self.Letterz`) false false)
    (set `/Game/JYP/Blueprints/BP_HighlightComp.bInteractable?` false (`self.BP_HighlightComp`))
    (set `self.bInteract?` false)
    (`SceneComponent.SetVisibility` (`self.ChildActor`) true false)))

(fn `UserConstructionScript`)