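; BP_D4 is a physical die actor, apparently four-sided, that can be rolled once across a table.
; Rolling disables table collision, randomizes rotation, raises the die and applies a random impulse.
; A recursive delayed position check detects when it settles, switching the die's collision object type while it moves.
; At rest, it re-enables table collision, sets a custom collision channel and turns off interaction and highlight interactability.
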(event `self.ReceiveBeginPlay`
  (set `self.bInteract?` true))

(event `Rolling`
  (if (`self.bInteract?`)
    (`/Game/JYP/Blueprints/BP_Table.CollisionDisabled` (`self.tableRef`))
    (`self.K2_SetActorRotation` (`KismetMathLibrary.MakeRotator` (`KismetMathLibrary.RandomFloatInRange` -180.0 180.0) (`KismetMathLibrary.RandomFloatInRange` -180.0 180.0) (`KismetMathLibrary.RandomFloatInRange` -180.0 180.0)))
    (`self.K2_SetActorLocation` (0.0 0.0 200.0))
    (`PrimitiveComponent.AddImpulse` (`self.Dice`) (`KismetMathLibrary.MakeVector` (`KismetMathLibrary.RandomFloatInRange` 100.0 1000.0) (`KismetMathLibrary.RandomFloatInRange` 100.0 1000.0) (`KismetMathLibrary.RandomFloatInRange` 100.0 1000.0)) "None" false)
    (`self.isStillRolling?`)
    (else
      (`PrimitiveComponent.SetCollisionObjectType` (`self.Dice`) "ECC_GameTraceChannel2"))))

(event `isStillRolling?`
  (set `self.diceLocation` (`self.K2_GetActorLocation`))
  (`KismetSystemLibrary.Delay` 0.5)
  (if (!= (`self.K2_GetActorLocation`) (`self.diceLocation`))
    (`self.isStillRolling?`)
    (`PrimitiveComponent.SetCollisionObjectType` (`self.Dice`) "ECC_WorldStatic")
    (else
      (`/Game/JYP/Blueprints/BP_Table.CollisionEnabled` (`self.tableRef`))
      (`PrimitiveComponent.SetCollisionObjectType` (`self.Dice`) "ECC_GameTraceChannel2")
      (set `/Game/JYP/Blueprints/BP_HighlightComp.bInteractable?` false (`self.BP_HighlightComp`))
      (set `self.bInteract?` false))))

(fn `UserConstructionScript`)