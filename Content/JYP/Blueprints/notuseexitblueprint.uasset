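; An exit prompt Blueprint that shows or hides its Text component through ExitTextOn and ExitTextOff events.
; The text starts hidden on BeginPlay, and nothing in this graph calls ExitTextOn.
; Every Tick it casts the player character to BP_JYPTestPlayer and hides the text while that player's ExitHere flag is false.
; The asset's name suggests it is unused.
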(event `self.ReceiveBeginPlay`
  (`SceneComponent.SetVisibility` (`self.Text`) false false))

(event `self.ReceiveTick`
  (params (DeltaSeconds :type "Float (single-precision)"))
  (bind _asbp_jyptest_player (cast `/Game/JYP/Blueprints/BP_JYPTestPlayer` (`GameplayStatics.GetPlayerCharacter` 0)))
  (if (not (`/Game/JYP/Blueprints/BP_JYPTestPlayer.bExitHere?` _asbp_jyptest_player))
    (`self.ExitTextOff`)))

(event `ExitTextOn`
  (`SceneComponent.SetVisibility` (`self.Text`) true false))

(event `ExitTextOff`
  (`SceneComponent.SetVisibility` (`self.Text`) false false))

(fn `UserConstructionScript`)