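; First-person test player for a tower game with letter interaction, turn-based monster encounters and level-to-level progression.
; A per-tick camera sphere trace outlines highlightable actors and detects letters, which right-click opens, and monsters.
; Number keys spend the player's turn on damage, healing or friendship while a monster is in view; the fourth is a stub.
; E opens the next floor by current level name, requiring a read letter in Opening.
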(event `Key|LeftMouseButton`
  (params (Key :type "Key Structure"))
  ;[1 1 1] Not use
)

(event `Key|E`
  (params (Key :type "Key Structure"))
  (:`Pressed`
    (if (`self.bPlayerCanPressNextDoor?`)
      (bind _returnvalue (`GameplayStatics.GetCurrentLevelName` true))
      (`|ExecutionSequence`
        (:`then_0`
          (if (`KismetStringLibrary.EqualEqual_StrStr` _returnvalue "Opening")
            (if (`self.bLetterTextHere?`)
              (`GameplayStatics.OpenLevel` "TowerLobbyFloor_Lobby"))))
        (:`then_1`
          (if (`KismetStringLibrary.EqualEqual_StrStr` _returnvalue "TowerLobbyFloor_Lobby")
            (`GameplayStatics.OpenLevel` "TowerFirstFloor_Normal")))
        (:`then_2`
          (if (`KismetStringLibrary.EqualEqual_StrStr` _returnvalue "TowerFirstFloor_Normal")
            (`GameplayStatics.OpenLevel` "TowerSecondFloor_Grace")))
        (:`then_3`
          (if (`KismetStringLibrary.EqualEqual_StrStr` _returnvalue "TowerSecondFloor_Grace")
            (`GameplayStatics.OpenLevel` "TowerThirdFloor_Life")))
        (:`then_4`
          (if (`KismetStringLibrary.EqualEqual_StrStr` _returnvalue "TowerThirdFloor_Life")
            (`GameplayStatics.OpenLevel` "TowerFourthFloor_Death")))
        (:`then_5`
          (if (`KismetStringLibrary.EqualEqual_StrStr` _returnvalue "TowerFourthFloor_Death")
            (`GameplayStatics.OpenLevel` "TowerLastFloor_Magician")))))))

(event `self.ReceiveTick`
  (params (DeltaSeconds :type "Float (single-precision)"))
  (bind _firstpersoncameracomponent (`self.FirstPersonCameraComponent`))
  (bind _returnvalue (`SceneComponent.K2_GetComponentLocation` _firstpersoncameracomponent))
  (bind (_outhit _returnvalue_2) (`KismetSystemLibrary.SphereTraceSingleForObjects` :`Start` _returnvalue :`End` (+ (* (`SceneComponent.GetForwardVector` _firstpersoncameracomponent) 1000.0) _returnvalue) :`Radius` 15.0 :`ObjectTypes` (`self.PlayerTrackingObjectTypes`) :`DrawDebugType` "ForOneFrame"))
  (if _returnvalue_2
    (`|ExecutionSequence`
      (:`then_0`
        (bind (_bblockinghit _binitialoverlap _time _distance _location _impactpoint _normal _impactnormal _physmat _hitactor) (`GameplayStatics.BreakHitResult` _outhit))
        (bind _returnvalue_3 (`self.GetComponentByClass` _hitactor "/Game/JYP/Blueprints/BP_HighlightComp.BP_HighlightComp_C"))
        (`/Engine/EditorBlueprintResources/StandardMacros.IsValid` _returnvalue_3
          (:`Is Valid`
            (`/Game/JYP/Blueprints/BP_HighlightComp.OnOutline` _returnvalue_3))))
      (:`then_1`
        (bind _asbp_letter (cast `/Game/JYP/Blueprints/BP_Letter` _hitactor))
        (set `self.bLetterHere?` true)
        (set `self.Letter` _asbp_letter))
      (:`then_2`
        (cast `/Game/JYP/Blueprints/Monster/BP_MonsterParent` _hitactor
          (:`then`
            (set `self.bPlayerSeeMonster?` true))
          (:`CastFailed`
            (set `self.bPlayerSeeMonster?` false)))))
    (else
      (set `self.bLetterHere?` false))))

(event `self.ReceiveBeginPlay`
  ;[1 1 1] Cache
  (bind _asbp_jypgmb (cast `/Game/JYP/Blueprints/BP_JYPGMB` (`GameplayStatics.GetGameMode`)))
  (set `self.JYPGMB` _asbp_jypgmb))

(event `Key|RightMouseButton`
  (params (Key :type "Key Structure"))
  (bind _letter (`self.Letter`))
  (:`Pressed`
    (if (`self.bLetterHere?`)
      (if (`/Game/JYP/Blueprints/BP_Letter.bInteract?` _letter)
        (`/Game/JYP/Blueprints/BP_Letter.WhenClickLetter` _letter)
        (set `self.bLetterTextHere?` true))
      (else
        (`KismetSystemLibrary.PrintString` "retry!")))))

(event `Key|One`
  (params (Key :type "Key Structure"))
  (bind _healthcomp (`self.HealthComp`))
  ;[1 1 1] Attack
  ;;[1 1 1] death
  (:`Pressed`
    (if (`self.bPlayerSeeMonster?`)
      (if (`/Game/JYP/Blueprints/BP_HealthComp.bAmIDie?` _healthcomp)
        _
        (elif (`self.bPlayerTurn?`)
          (`/Game/JYP/Blueprints/BP_HealthComp.Damaged` _healthcomp (`self.damage`))
          (set `self.bPlayerTurn?` false)))
      (else
        (`KismetSystemLibrary.PrintString` "No Enemy Interaction.")))))

(event `Key|Two`
  (params (Key :type "Key Structure"))
  ;[1 1 1] Attack
  ;;[1 1 1] life
  (:`Pressed`
    (if (`self.bPlayerSeeMonster?`)
      (if (`self.bPlayerTurn?`)
        (`/Game/JYP/Blueprints/BP_HealthComp.Healing` (`self.BP_HealthComp`) (`self.heal`))
        (set `self.bPlayerTurn?` false)))))

(event `Key|Three`
  (params (Key :type "Key Structure"))
  ;[1 1 1] Attack
  ;;[1 1 1] grace
  (:`Pressed`
    (if (`self.bPlayerSeeMonster?`)
      (if (`self.bPlayerTurn?`)
        (`/Game/JYP/Blueprints/BP_FriendshipComp.GetFriendship` (`self.FriendshipComp`) (`self.friendship`))
        (set `self.bPlayerTurn?` false)))))

(event `Key|Four`
  (params (Key :type "Key Structure"))
  ;[1 1 1] Attack
  ;;[1 1 1] normal
  (:`Pressed`
    (if (`self.bPlayerSeeMonster?`)
      (if (`self.bPlayerTurn?`)
        _))))

(fn `UserConstructionScript`)