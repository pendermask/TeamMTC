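; BP_HighlightComp is a component that briefly outlines its owning actor's static mesh when OnOutline fires and Interactable is true.
; It spawns a movable, collision-free StaticMeshActor copy at the owner mesh's transform, with a very short lifespan, so each outline clears itself.
; The copy's first material slot gets a dynamic MAT_Outline instance driven by the component's OutlineColor and Thickness.
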(event `OnOutline`
  (bind _returnvalue (`Actor.GetComponentByClass` (`self.GetOwner`) "/Script/Engine.StaticMeshComponent"))
  (if (`self.bInteractable?`)
    (bind _returnvalue_2 (`|SpawnActorFromClass` "/Script/Engine.StaticMeshActor" (`SceneComponent.K2_GetComponentToWorld` _returnvalue) "Undefined" "OverrideRootScale" null null))
    (`StaticMeshActor.SetMobility` _returnvalue_2 "Movable")
    (`Actor.SetLifeSpan` _returnvalue_2 0.1)
    (`Actor.SetActorEnableCollision` _returnvalue_2 false)
    (bind _staticmeshcomponent (`StaticMeshActor.StaticMeshComponent` _returnvalue_2))
    (`StaticMeshComponent.SetStaticMesh` _staticmeshcomponent (`StaticMeshComponent.StaticMesh` _returnvalue))
    (bind _returnvalue_3 (`PrimitiveComponent.CreateDynamicMaterialInstance` _staticmeshcomponent 0 "/Game/JYP/Assets/Material/MAT_Outline.MAT_Outline" "None"))
    (`MaterialInstanceDynamic.SetVectorParameterValue` _returnvalue_3 "color" (`self.outlineColor`))
    (`MaterialInstanceDynamic.SetScalarParameterValue` _returnvalue_3 "thickness" (`self.thickness`))))