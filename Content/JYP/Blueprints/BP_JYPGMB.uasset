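; BP_JYPGMB appears to be a game mode that runs turn-based card combat between the player and the current enemy.
; BeginPlay caches the player and gives them the first turn flag, while PlayerTurn restarts their turn through CardGame.
; CardGame times the player's turn with a timeline, then calls OnMyturn on the monster in CurrentEnemy's child actor.
; A separate event spawns a teleport door at a given transform after a monster dies.
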(event `SpawnTeleportDoor`
  (params (NewParam :type "Transform Structure"))
  ;[1 1 1] spawn door after monster dead
  (`|SpawnActorFromClass` "/Game/JYP/Blueprints/BP_TeleportDoor.BP_TeleportDoor_C" NewParam "Undefined" "OverrideRootScale" null null))

(event `self.ReceiveBeginPlay`
  (bind _asbp_jyptest_player (cast `/Game/JYP/Blueprints/BP_JYPTestPlayer` (`GameplayStatics.GetPlayerCharacter` 0)))
  (bind _output_get (set `self.Player` _asbp_jyptest_player))
  (bind _returnvalue (`GameplayStatics.GetCurrentLevelName` true))
  (bind _output_get_2 (set `/Game/JYP/Blueprints/BP_JYPTestPlayer.bPlayerTurn?` true _output_get)))

(event `PlayerTurn`
  (set `/Game/JYP/Blueprints/BP_JYPTestPlayer.bPlayerTurn?` true (`self.Player`))
  (`self.CardGame`))

(event `CardGame`
  (if (`/Game/JYP/Blueprints/BP_JYPTestPlayer.bPlayerTurn?` (`self.Player`))
    (`Timeline|Timeline_0` :!via `PlayFromStart`
      (:`Finished`
        (set `/Game/JYP/Blueprints/BP_JYPTestPlayer.bPlayerTurn?` false (`self.Player`))
        (`self.CardGame`)))
    (else
      (bind _asbp_monster_parent (cast `/Game/JYP/Blueprints/Monster/BP_MonsterParent` (`ChildActorComponent.ChildActor` (`self.currentEnemy`))))
      (`/Game/JYP/Blueprints/Monster/BP_MonsterParent.OnMyturn` _asbp_monster_parent))))

(fn `UserConstructionScript`)