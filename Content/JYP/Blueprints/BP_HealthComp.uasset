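; BP_HealthComp is a health component that tracks its owner's HP and handles its death.
; BeginPlay caches the BP_JYPGMB game mode and the player character, and sets current health to max.
; Damaged subtracts card damage, printing the remaining HP or calling Dead at zero or below.
; Dead has the game mode spawn a teleport door at the owner's location and rotation, then destroys the owner.
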(event `self.ReceiveBeginPlay`
  (bind _asbp_jypgmb (cast `/Game/JYP/Blueprints/BP_JYPGMB` (`GameplayStatics.GetGameMode`)))
  (set `self.JYPGMB` _asbp_jypgmb)
  (bind _output_get (set `self.currenthealth` (`self.maxHealth`)))
  (`KismetSystemLibrary.PrintString` (`KismetStringLibrary.Concat_StrStr` "my hp is " (`KismetStringLibrary.Conv_IntToString` _output_get)))
  (bind _asbp_jyptest_player (cast `/Game/JYP/Blueprints/BP_JYPTestPlayer` (`GameplayStatics.GetPlayerCharacter` 0)))
  (set `self.Player` _asbp_jyptest_player))

(event `Dead`
  (bind _returnvalue (`self.GetOwner`))
  (bind (_returnvalue_location _returnvalue_rotation) (`KismetMathLibrary.BreakTransform` (`Actor.GetTransform` _returnvalue)))
  (`/Game/JYP/Blueprints/BP_JYPGMB.SpawnTeleportDoor` (`self.JYPGMB`) (`KismetMathLibrary.MakeTransform` _returnvalue_location _returnvalue_rotation))
  (`Actor.K2_DestroyActor` _returnvalue))

(event `Damaged`
  (params (CardDamage :type Integer))
  (bind _output_get (set `self.currenthealth` (- (`self.currenthealth`) CardDamage)))
  (if (<= _output_get 0)
    (`self.Dead`)
    (else
      (`KismetSystemLibrary.PrintString` (`KismetStringLibrary.Conv_IntToString` _output_get)))))