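; Dice table actor that turns the dice component landing in its trigger box into the monster type, then opens a random numbered level.
; On BeginPlay it disables box collision, reads the stored type from GI_GameInstance and slides the table via a flip-flopped Timeline.
; A Dice overlap disables the box, waits briefly, then saves the component name's suffix to the game instance before the level load.
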(event `self.ReceiveBeginPlay`
  (`|ExecutionSequence`
    (:`then_0`
      (`self.CollisionDisabled`))
    (:`then_1`
      (bind _asgi_game_instance (cast `/Game/JYP/Blueprints/GI_GameInstance` (`GameplayStatics.GetGameInstance`))
        (:`then`
          (`/Engine/EditorBlueprintResources/StandardMacros.IsValid` _asgi_game_instance
            (:`Is Valid`
              (set `self.currentMonsterType` (`/Game/JYP/Blueprints/GI_GameInstance.GI_Type` _asgi_game_instance)))
            (:`Is Not Valid`
              (`KismetSystemLibrary.PrintString` "fail to cast" :!label _label))))
        (:`CastFailed`
          (goto _label))))
    (:`then_2`
      (if true
        (`self.TableUpdate`)))))

(event `TableUpdate`
  ;[0 0 0 0 25] Table Update When Init
  (`/Engine/EditorBlueprintResources/StandardMacros.FlipFlop`
    (:`A`
      (bind (_direction _tableupdate) (`Timeline|TableUpdating` :!label _label_2)
        (:`Update`
          (`SceneComponent.K2_SetRelativeLocation` (`self.Table`) (`KismetMathLibrary.VLerp` (`self.StartTableVector`) (`self.TargetTableVector`) _tableupdate) false false))))
    (:`B`
      (goto _label_2 :!via `Reverse`))))

(event `self.Box.OnComponentBeginOverlap`
  (params (OverlappedComponent :type "PrimitiveComponent Object Reference") (OtherActor :type "Actor Object Reference") (OtherComp :type "PrimitiveComponent Object Reference") (OtherBodyIndex :type Integer) (bFromSweep :type Boolean) (SweepResult :type "HitResult Structure (by ref)"))
  (bind _returnvalue (`KismetSystemLibrary.GetDisplayName` OtherComp))
  (if (== OtherActor (`self.dice`))
    (`KismetSystemLibrary.PrintString` _returnvalue)
    (bind _output_get (set `self.currentMonsterType` _returnvalue))
    (`self.CollisionDisabled`)
    (`KismetSystemLibrary.Delay` 1.0)
    (bind _asgi_game_instance (cast `/Game/JYP/Blueprints/GI_GameInstance` (`GameplayStatics.GetGameInstance`))
      (:`then`
        (`/Engine/EditorBlueprintResources/StandardMacros.IsValid` _asgi_game_instance
          (:`Is Valid`
            (bind _output_get_2 (set `/Game/JYP/Blueprints/GI_GameInstance.GI_Type` (`.RightS` (`KismetStringLibrary.Split` _output_get ".")) _asgi_game_instance))
            (`KismetSystemLibrary.PrintString` _output_get_2)
            (`GameplayStatics.OpenLevel` (`KismetStringLibrary.Conv_StringToName` (`KismetStringLibrary.Conv_IntToString` (`KismetMathLibrary.RandomIntegerInRange` 0 4)))))
          (:`Is Not Valid`
            (`KismetSystemLibrary.PrintString` "retry, is not valid" :!label _label_3))))
      (:`CastFailed`
        (goto _label_3)))))

(event `CollisionEnabled`
  (`PrimitiveComponent.SetCollisionEnabled` (`self.Box`) "QueryAndPhysics"))

(event `CollisionDisabled`
  (`PrimitiveComponent.SetCollisionEnabled` (`self.Box`) "NoCollision"))

(fn `OnRep_dice`)

(fn `UserConstructionScript`)