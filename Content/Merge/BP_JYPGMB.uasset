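; BP_JYPGMB, apparently a game mode, runs the turn flow of a card battle between the player and a monster.
; On BeginPlay it caches the game instance, player and current enemy's monster, giving the player the first turn.
; CardGame plays a timeline for the player's turn, increments the game instance's action count, then calls the monster's OnMyturn; PlayerTurn hands control back.
; A separate event spawns a teleport door, intended for after monster death.
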(event `SpawnTeleportDoor`
  (params (NewParam :type "Transform Structure"))
  ;[1 1 1] spawn door after monster dead
  (`|SpawnActorFromClass` "/Game/JYP/Blueprints/BP_TeleportDoor.BP_TeleportDoor_C" NewParam "Undefined" "OverrideRootScale" null null))

(event `self.ReceiveBeginPlay`
  (bind _currentenemy (`self.currentEnemy`))
  ;[1 1 1] Caching
  (bind _asgi_game_instance (cast `/Game/JYP/Blueprints/GI_GameInstance` (`GameplayStatics.GetGameInstance`)))
  (set `self.GameInstance` _asgi_game_instance)
  (bind _asbp_jyptest_player (cast `/Game/JYP/Blueprints/BP_JYPTestPlayer` (`GameplayStatics.GetPlayerCharacter` 0)))
  (bind _output_get (set `self.Player` _asbp_jyptest_player))
  (`GameplayStatics.GetCurrentLevelName` true)
  (`/Engine/EditorBlueprintResources/StandardMacros.IsValid` _currentenemy
    (:`Is Valid`
      (set `/Game/JYP/Blueprints/BP_JYPTestPlayer.bPlayerTurn?` true _output_get)
      (bind _asbp_monster_parent (cast `/Game/JYP/Blueprints/Monster/BP_MonsterParent` (`ChildActorComponent.ChildActor` _currentenemy)))
      (set `self.MonsterParent` _asbp_monster_parent))))

(event `CardGame`
  (bind _gameinstance (`self.GameInstance`))
  ;[1 1 1] Turn
  (`/Engine/EditorBlueprintResources/StandardMacros.IsValid` (`self.MonsterParent`)
    (:`Is Valid`
      (if (`/Game/JYP/Blueprints/BP_JYPTestPlayer.bPlayerTurn?` (`self.Player`))
        (`Timeline|Timeline_0` :!via `PlayFromStart`
          (:`Finished`
            (set `/Game/JYP/Blueprints/BP_JYPTestPlayer.bPlayerTurn?` false (`self.Player`))
            (bind _output_get (set `/Game/JYP/Blueprints/GI_GameInstance.playerActionCount` (+ (`/Game/JYP/Blueprints/GI_GameInstance.playerActionCount` _gameinstance) 1) _gameinstance))
            (`KismetSystemLibrary.PrintString` (`KismetStringLibrary.Conv_IntToString` _output_get))
            (`self.CardGame`)))
        (else
          (`/Game/JYP/Blueprints/Monster/BP_MonsterParent.OnMyturn` (`self.MonsterParent`)))))))

(event `PlayerTurn`
  ;[1 1 1] Turn
  (set `/Game/JYP/Blueprints/BP_JYPTestPlayer.bPlayerTurn?` true (`self.Player`))
  (`self.CardGame`))

(fn `UserConstructionScript`)