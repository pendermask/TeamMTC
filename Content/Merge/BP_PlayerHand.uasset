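; Hand-tracking player for a card game, where cards are drawn, grabbed and shot at the monster spawner.
; CardsOn spawns a four-card hand above the left palm; Grab1-4 select a child card that Tick holds over the right palm, yawed from the camera.
; ShootCard attaches a name-matched particle, moves the card to the spawner and destroys it.
; P saves a right-hand gesture; the two-hand Interaction only prints a placeholder.
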(event `self.ReceiveBeginPlay`
  (`HeadMountedDisplayFunctionLibrary.SetTrackingOrigin` "Floor"))

(event `Key|P`
  (params (Key :type "Key Structure"))
  (:`Pressed`
    (`HTHandTrackingGestureComponent.SaveGesture` (`self.HTHandTrackingGesture`) "/Game/HOO/Gesture/RHG_Interaction.RHG_Interaction" "Right" false (-1.0 -1.0 -1.0))
    (`KismetSystemLibrary.PrintString` "Saved")))

(event `self.ReceiveTick`
  (params (DeltaSeconds :type "Float (single-precision)"))
  (bind (_returnvalue_x _returnvalue_y _returnvalue_z) (`KismetMathLibrary.BreakVector` (`HandTrackingFL.GetHandPalmLocation` (`self.RightHandTracking`))))
  (bind _returnvalue (`KismetMathLibrary.MakeVector` _returnvalue_x _returnvalue_y (+ _returnvalue_z 20.0)))
  (bind (_returnvalue_roll _returnvalue_pitch _returnvalue_yaw) (`KismetMathLibrary.BreakRotator` (`KismetMathLibrary.Conv_VectorToRotator` (- _returnvalue (`SceneComponent.K2_GetComponentLocation` (`self.Camera`))))))
  (`|ExecutionSequence`
    (:`then_0`
      (if (and (`self.GrabOn?`) (not (`self.ShootCard?`)))
        (bind (_sweephitresult _returnvalue_2) (`self.K2_SetActorTransform` (`self.GrabbedCard`) (`KismetMathLibrary.MakeTransform` _returnvalue (`KismetMathLibrary.MakeRotator` _returnvalue_roll 0.0 (+ _returnvalue_yaw 90.0))) false false))
        (set `self.OnRightHand` _returnvalue_2)))))

(event `Initialize`
  (if (not (`self.OnRightHand`))
    (set `self.InitializeCards` true)
    (if (`self.PlayStart`)
      (`self.K2_DestroyActor` (stale `CardsOn` _returnvalue_2)))
    (set `self.CardsOn?` false)))

(event `Grab1`
  (if (`self.CardsOn?`)
    (set `self.GrabOn?` true)
    (bind _returnvalue (`GameplayStatics.GetActorOfClass` "/Game/HOO/BP_HandCardSpawn_1.BP_HandCardSpawn_1_C"))
    (bind _returnvalue_2 (`GameplayStatics.GetActorOfClass` (`ChildActorComponent.ChildActorClass` (`/Game/HOO/BP_HandCardSpawn_1.Child1` _returnvalue))))
    (set `self.GrabbedCard` _returnvalue_2)))

(event `Left_Interaction`
  (bind _output_get (set `self.L_Interaction` true))
  (if (stale `Right_Interaction` _output_get)
    (`self.Interaction`)))

(event `CardsOn`
  (bind (_returnvalue_x _returnvalue_y _returnvalue_z) (`KismetMathLibrary.BreakVector` (`HandTrackingFL.GetHandPalmLocation` (`self.LeftHandTracking`))))
  (bind _returnvalue (`KismetMathLibrary.MakeVector` _returnvalue_x _returnvalue_y (+ _returnvalue_z 20.0)))
  (bind (_returnvalue_roll _returnvalue_pitch _returnvalue_yaw) (`KismetMathLibrary.BreakRotator` (`KismetMathLibrary.Conv_VectorToRotator` (- _returnvalue (`SceneComponent.K2_GetComponentLocation` (`self.Camera`))))))
  (if (`self.CardsOn?`)
    _
    (elif (`self.InitializeCards`)
      (bind _returnvalue_2 (`|SpawnActorFromClass` "/Game/HOO/BP_HandCardSpawn_1.BP_HandCardSpawn_1_C" (`KismetMathLibrary.MakeTransform` _returnvalue (`KismetMathLibrary.MakeRotator` _returnvalue_roll 0.0 (+ _returnvalue_yaw 90.0))) "Undefined" "OverrideRootScale" null null))
      (set `self.PlayStart` true)
      (set `self.CardsOn?` true)
      (set `self.InitializeCards` false))))

(event `Right_Interaction`
  (bind _output_get (set `self.R_Interaction` true))
  (if (stale `Left_Interaction` _output_get)
    (`self.Interaction`)))

(event `Grab2`
  (if (`self.CardsOn?`)
    (set `self.GrabOn?` true)
    (bind _returnvalue (`GameplayStatics.GetActorOfClass` "/Game/HOO/BP_HandCardSpawn_1.BP_HandCardSpawn_1_C"))
    (bind _returnvalue_2 (`GameplayStatics.GetActorOfClass` (`ChildActorComponent.ChildActorClass` (`/Game/HOO/BP_HandCardSpawn_1.Child2` _returnvalue))))
    (set `self.GrabbedCard` _returnvalue_2)))

(event `Interaction`
  (`KismetSystemLibrary.PrintString` "Hello"))

(event `Grab3`
  (if (`self.CardsOn?`)
    (set `self.GrabOn?` true)
    (bind _returnvalue (`GameplayStatics.GetActorOfClass` "/Game/HOO/BP_HandCardSpawn_1.BP_HandCardSpawn_1_C"))
    (bind _returnvalue_2 (`GameplayStatics.GetActorOfClass` (`ChildActorComponent.ChildActorClass` (`/Game/HOO/BP_HandCardSpawn_1.Child3` _returnvalue))))
    (set `self.GrabbedCard` _returnvalue_2)))

(event `CardsOff`
  (if (`self.CardsOn?`)
    (`self.K2_DestroyActor` (stale `CardsOn` _returnvalue_2))
    (set `self.CardsOn?` false)))

(event `Grab4`
  (if (`self.CardsOn?`)
    (set `self.GrabOn?` true)
    (bind _returnvalue (`GameplayStatics.GetActorOfClass` "/Game/HOO/BP_HandCardSpawn_1.BP_HandCardSpawn_1_C"))
    (bind _returnvalue_2 (`GameplayStatics.GetActorOfClass` (`ChildActorComponent.ChildActorClass` (`/Game/HOO/BP_HandCardSpawn_1.Child4` _returnvalue))))
    (set `self.GrabbedCard` _returnvalue_2)))

(event `ShootCard`
  (bind _grabbedcard (`self.GrabbedCard`))
  (bind _rootcomponent (`Actor.RootComponent` _grabbedcard))
  (bind (_value _returnvalue) (`BlueprintMapLibrary.Map_Find` (`self.particles`) (`KismetStringLibrary.Split` (`KismetSystemLibrary.GetDisplayName` _grabbedcard) "-")))
  (if (`self.GrabOn?`)
    (set `self.ShootCard?` true)
    (bind _returnvalue_2 (`GameplayStatics.GetActorOfClass` "/Game/HOO/Monster/BP_hoo_MonsterSpawner.BP_hoo_MonsterSpawner_C"))
    (if _returnvalue
      (`GameplayStatics.SpawnEmitterAttached` _value _rootcomponent "None" (0.0 0.0 0.0) (struct) (0.5 0.5 0.5))
      (set `self.makeTransform` (`self.GetTransform` (`self.GetParentActor` (`self.GrabbedCard`))))
      (`KismetSystemLibrary.MoveComponentTo` _rootcomponent (`KismetMathLibrary.InverseTransformLocation` (`self.makeTransform`) (+ (`self.K2_GetActorLocation` _returnvalue_2) (0.0 0.0 150.0))) (`KismetMathLibrary.MakeRotFromY` (`self.GetActorRightVector` _grabbedcard)) false false 3.0 true)
      (`KismetSystemLibrary.PrintString` (`KismetSystemLibrary.GetObjectName` _grabbedcard))
      (bind _returnvalue_3 (`GameplayStatics.GetActorOfClass` "/Game/HOO/Cards/BP_CardParents.BP_CardParents_C"))
      (`KismetSystemLibrary.PrintString` (`KismetStringLibrary.Conv_IntToString` (`/Game/HOO/Cards/BP_CardParents.Value` _returnvalue_3)))
      (`KismetSystemLibrary.PrintString` (`/Game/HOO/Cards/BP_CardParents.Type` _returnvalue_3))
      (`KismetSystemLibrary.PrintString` "MOCE COMPLETE")
      (set `self.GrabOn?` false)
      (set `self.CardsOn?` false)
      (`self.K2_DestroyActor` (`self.GrabbedCard`))
      (set `self.ShootCard?` false)
      (set `self.OnRightHand` false)
      (else
        (`KismetSystemLibrary.PrintString` "EMITTER ERROR")))))

(event `GrabCancel`
  (if (`self.GrabOn?`)
    (`self.K2_DestroyActor` (`self.GrabbedCard`))
    (set `self.CardsOn?` false)
    (set `self.GrabOn?` false)
    (set `self.OnRightHand` false)))

(fn `UserConstructionScript`)