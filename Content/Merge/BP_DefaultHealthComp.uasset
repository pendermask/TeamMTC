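; Health component shared by the hand-tracking player and monsters, handling damage, healing and death.
; Player health lives in the game instance, while monsters track a local value against their max.
; Damage plays hit effects; both death paths increment the dead-monster counter, including the player's.
; Player death opens the lobby level; monster death spawns a teleport door via the game mode, enables door pressing and destroys the owner.
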(event `self.ReceiveBeginPlay`
  ;[0 0 0 0 50] Caching
  (bind _asgi_dgame_instance (cast `/Game/Merge/GI_DGameInstance` (`GameplayStatics.GetGameInstance`)))
  (set `self.GameInstance` _asgi_dgame_instance)
  (bind _asbp_gmb (cast `/Game/Merge/BP_GMB` (`GameplayStatics.GetGameMode`)))
  (set `self.GMB` _asbp_gmb)
  (set `self.currenthealth` (`self.maxHealth`))
  (bind _asbp_default_hand_tracking_player (cast `/Game/Merge/BP_DefaultHandTrackingPlayer` (`GameplayStatics.GetPlayerPawn` 0)))
  (set `self.Player` _asbp_default_hand_tracking_player))

(event `Dead`
  (bind (_returnvalue_location _returnvalue_rotation) (`KismetMathLibrary.BreakTransform` (`Actor.GetTransform` (`self.GetOwner`))))
  ;[0 0 0 0 50] Dead
  (if (== (`self.GetOwner`) (`self.Player`))
    (`GameplayStatics.OpenLevel` "DefaultTowerLobbyFloor_Lobby")
    (else
      (`/Game/Merge/BP_GMB.SpawnTeleportDoor` (`self.GMB`) (`KismetMathLibrary.MakeTransform` _returnvalue_location _returnvalue_rotation))
      (set `/Game/Merge/BP_DefaultHandTrackingPlayer.bPlayerCanPressNextDoor?` true (`self.Player`))
      (`Actor.K2_DestroyActor` (`self.GetOwner`)))))

(event `Damaged`
  (params (GetDamage :type Integer))
  ;[0 0 0 0 50] Damaged
  (set `self.getDamage` GetDamage)
  (`GameplayStatics.SpawnEmitterAttached` "/Game/Asset/Particle/P_Hit.P_Hit" (`Actor.RootComponent` (`self.GetOwner`)) "None" (0.0 0.0 0.0) (struct) (10.0 10.0 10.0))
  (`GameplayStatics.PlaySound2D` "/Game/Asset/Sound/CardPlay/playerDamage.playerDamage" 10.0 1.0 0.0 null null)
  (if (== (`self.GetOwner`) (`GameplayStatics.GetPlayerPawn` 0))
    (bind _output_get (set `/Game/Merge/GI_DGameInstance.playerHealth` (- (`/Game/Merge/GI_DGameInstance.playerHealth` (`self.GameInstance`)) (`self.getDamage`)) (`self.GameInstance`)))
    (if (<= _output_get 0)
      (set `self.bAmIDie?` true :!label _label)
      (set `/Game/Merge/GI_DGameInstance.deadMonsterCount` (+ (`/Game/Merge/GI_DGameInstance.deadMonsterCount` (`self.GameInstance`)) 1) (`self.GameInstance`))
      (`self.Dead`))
    (else
      (bind _output_get_2 (set `self.currenthealth` (- (`self.currenthealth`) (`self.getDamage`))))
      (if (<= _output_get_2 0)
        (set `self.bMonsterDamaged?` true)
        (goto _label)))))

(event `Healing`
  (params (GetHealing :type Integer))
  ;[0 0 0 0 50] Healing
  (set `self.getHealing` GetHealing)
  (if (== (`self.GetOwner`) (`GameplayStatics.GetPlayerPawn` 0))
    ;;[0 0 0 0 20] player healing
    (bind _output_get (set `/Game/Merge/GI_DGameInstance.playerHealth` (+ (`self.getHealing`) (`/Game/Merge/GI_DGameInstance.playerHealth` (`self.GameInstance`))) (`self.GameInstance`)))
    (if (> _output_get 30)
      (set `/Game/Merge/GI_DGameInstance.playerHealth` 30 (`self.GameInstance`)))
    (`TextRenderComponent.K2_SetText` (`/Game/Merge/BP_DefaultHandTrackingPlayer.HP` (`self.Player`)) (`KismetTextLibrary.Conv_IntToText` (`/Game/Merge/GI_DGameInstance.playerHealth` (`self.GameInstance`))))
    (else
      ;;[0 0 0 0 20] monster healing
      (bind _output_get_2 (set `self.currenthealth` (+ (`self.getHealing`) (`self.currenthealth`))))
      (if (> _output_get_2 (`self.maxHealth`))
        (set `self.currenthealth` (`self.maxHealth`))))))