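; BP_DefaultTeleportDoor is a door that fades in a level-specific card on BeginPlay in every level except MOpening.
; It blocks the hand-tracking player's next-door press and shows its mesh and plane.
; The current level's name suffix, or the GameInstance's previous level on MEscapeFloor, picks a material from LevelNameFilter.
; A timeline animates that dynamic material's Opacity, then lets the player open the card.
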(event `self.ReceiveBeginPlay`
  (bind (_lefts _rights) (`KismetStringLibrary.Split` (`self.currentLevel`) "_"))
  (bind (_value _returnvalue) (`BlueprintMapLibrary.Map_Find` (`self.levelNameFilter`) _rights))
  (bind _returnvalue_2 (`GameplayStatics.GetCurrentLevelName` true))
  (if (not (`KismetStringLibrary.EqualEqual_StrStr` _returnvalue_2 "MOpening"))
    (bind _asbp_default_hand_tracking_player (cast `/Game/Merge/BP_DefaultHandTrackingPlayer` (`GameplayStatics.GetPlayerPawn` 0)))
    (bind _output_get (set `self.Player` _asbp_default_hand_tracking_player))
    (set `/Game/Merge/BP_DefaultHandTrackingPlayer.bPlayerCanPressNextDoor?` false _output_get)
    (`SceneComponent.SetVisibility` (`self.StaticMesh`) true false)
    (`SceneComponent.SetVisibility` (`self.Plane`) true false)
    (bind _returnvalue_3 (`GameplayStatics.GetCurrentLevelName` true))
    (bind _output_get_2 (set `self.currentLevel` _returnvalue_3))
    (if (`KismetStringLibrary.EqualEqual_StrStr` _output_get_2 "MEscapeFloor")
      (bind _asgi_dgame_instance (cast `/Game/Merge/GI_DGameInstance` (`GameplayStatics.GetGameInstance`)))
      (bind _previouslevel (`/Game/Merge/GI_DGameInstance.previousLevel` _asgi_dgame_instance))
      (`KismetSystemLibrary.PrintString` _previouslevel)
      (bind (_lefts_2 _rights_2) (`KismetStringLibrary.Split` _previouslevel "_"))
      (`KismetSystemLibrary.PrintString` _rights_2)
      (bind (_value_2 _returnvalue_4) (`BlueprintMapLibrary.Map_Find` (`self.levelNameFilter`) _rights_2))
      (bind _returnvalue_5 (`PrimitiveComponent.CreateDynamicMaterialInstance` (`self.Plane`) 0 _value_2 "None"))
      (if _returnvalue_4
        (bind (_direction _appearance) (`Timeline|Timeline_0` :!via `PlayFromStart`)
          (:`Update`
            (`MaterialInstanceDynamic.SetScalarParameterValue` _returnvalue_5 "Opacity" _appearance))
          (:`Finished`
            (set `/Game/Merge/BP_DefaultHandTrackingPlayer.bPlayerCanCardOpen?` true (`self.Player`)))))
      (else
        (`KismetSystemLibrary.PrintString` _rights)
        (if _returnvalue
          (bind _returnvalue_6 (`PrimitiveComponent.CreateDynamicMaterialInstance` (`self.Plane`) 0 _value "None"))
          (bind (_direction_2 _appearance_2) (`Timeline|CardAppearance` :!via `PlayFromStart`)
            (:`Update`
              (`MaterialInstanceDynamic.SetScalarParameterValue` _returnvalue_6 "Opacity" _appearance_2))
            (:`Finished`
              (set `/Game/Merge/BP_DefaultHandTrackingPlayer.bPlayerCanCardOpen?` true (`self.Player`)))))))))

(fn `UserConstructionScript`)