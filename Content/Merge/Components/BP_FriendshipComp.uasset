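; BP_FriendshipComp is a component that tracks a monster's friendship value and feeds it into a game-wide total.
; BeginPlay caches GI_GameInstance; GetFriendship adds a random amount, up to its input, to the monster's value.
; When a random key exists in FriendshipDialogue, the accumulated value is added to TotalFriendship and printed with dialogue.
; The increment, key check and printed lookup use separate random evaluations, so they can differ.
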(event `self.ReceiveBeginPlay`
  ;[1 1 1] Comment
  (bind _asgi_game_instance (cast `/Game/JYP/Blueprints/GI_GameInstance` (`GameplayStatics.GetGameInstance`)))
  (set `self.GameInstance` _asgi_game_instance))

(event `GetFriendship`
  (params (friendship :type Integer))
  (bind _returnvalue (`KismetMathLibrary.RandomIntegerInRange` 0 friendship))
  (bind _gameinstance (`self.GameInstance`))
  (bind (_value _returnvalue_2) (`BlueprintMapLibrary.Map_Find` (`self.friendshipDialogue`) _returnvalue))
  (bind _output_get (set `self.eachMonsterFriendshipValue` (+ (`self.eachMonsterFriendshipValue`) _returnvalue)))
  (if _returnvalue_2
    (set `/Game/JYP/Blueprints/GI_GameInstance.totalFriendship` (+ (`/Game/JYP/Blueprints/GI_GameInstance.totalFriendship` _gameinstance) _output_get) _gameinstance)
    (`KismetSystemLibrary.PrintString` (`KismetStringLibrary.Concat_StrStr` "friendship : " (`KismetStringLibrary.Conv_IntToString` _output_get) " \n" _value))))