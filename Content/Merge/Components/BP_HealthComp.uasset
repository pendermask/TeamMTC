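; Health component that tracks damage, healing and death for its owning actor, apparently a monster.
; BeginPlay fills health to maximum and caches the game instance, game mode and player.
; Damaged subtracts health and, at zero or below, increments the game instance's dead monster count and calls Dead, which has the game mode spawn a teleport door at the owner's location before destroying it.
; Healing adds health, capped at maximum.
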(event `self.ReceiveBeginPlay`
  (bind _asgi_game_instance (cast `/Game/JYP/Blueprints/GI_GameInstance` (`GameplayStatics.GetGameInstance`)))
  (set `self.GameInstance` _asgi_game_instance)
  (bind _asbp_jypgmb (cast `/Game/JYP/Blueprints/BP_JYPGMB` (`GameplayStatics.GetGameMode`)))
  (set `self.JYPGMB` _asbp_jypgmb)
  (bind _output_get (set `self.currenthealth` (`self.maxHealth`)))
  (bind _asbp_jyptest_player (cast `/Game/JYP/Blueprints/BP_JYPTestPlayer` (`GameplayStatics.GetPlayerCharacter` 0)))
  (set `self.Player` _asbp_jyptest_player))

(event `Dead`
  (bind _returnvalue (`self.GetOwner`))
  (bind (_returnvalue_location _returnvalue_rotation) (`KismetMathLibrary.BreakTransform` (`Actor.GetTransform` _returnvalue)))
  (`/Game/JYP/Blueprints/BP_JYPGMB.SpawnTeleportDoor` (`self.JYPGMB`) (`KismetMathLibrary.MakeTransform` _returnvalue_location _returnvalue_rotation))
  (`Actor.K2_DestroyActor` _returnvalue))

(event `Damaged`
  (params (GetDamage :type Integer))
  (bind _gameinstance (`self.GameInstance`))
  ;[1 1 1] Comment
  (bind _output_get (set `self.currenthealth` (- (`self.currenthealth`) GetDamage)))
  (if (<= _output_get 0)
    (set `self.bAmIDie?` true)
    (set `/Game/JYP/Blueprints/GI_GameInstance.deadMonsterCount` (+ (`/Game/JYP/Blueprints/GI_GameInstance.deadMonsterCount` _gameinstance) 1) _gameinstance)
    (`self.Dead`)))

(event `Healing`
  (params (GetHealing :type Integer))
  (bind _maxhealth (`self.maxHealth`))
  ;[1 1 1] Comment
  (bind _output_get (set `self.currenthealth` (+ GetHealing (`self.currenthealth`))))
  (if (> _output_get _maxhealth)
    (bind _output_get_2 (set `self.currenthealth` _maxhealth))))