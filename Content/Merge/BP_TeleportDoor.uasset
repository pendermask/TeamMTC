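; Teleport door actor that fades in a level-specific card on its plane at BeginPlay, locking the player's next-door input until the fade finishes.
; It looks up the card material by the level name's suffix after an underscore, using the game instance's previous level on JYPEscapeFloor and the current level elsewhere.
; Timelines animate the dynamic material's Opacity, then set PlayerCanPressNextDoor; no teleport logic lives here.
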(event `self.ReceiveBeginPlay`
  (bind (_lefts _rights) (`KismetStringLibrary.Split` (`self.currentLevel`) "_"))
  (bind (_value _returnvalue) (`BlueprintMapLibrary.Map_Find` (`self.levelNameFilter`) _rights))
  (bind _asbp_jyptest_player (cast `/Game/JYP/Blueprints/BP_JYPTestPlayer` (`GameplayStatics.GetPlayerCharacter` 0)))
  (bind _output_get (set `self.Player` _asbp_jyptest_player))
  (set `/Game/JYP/Blueprints/BP_JYPTestPlayer.bPlayerCanPressNextDoor?` false _output_get)
  (`SceneComponent.SetVisibility` (`self.StaticMesh`) true false)
  (`SceneComponent.SetVisibility` (`self.Plane`) true false)
  (bind _returnvalue_2 (`GameplayStatics.GetCurrentLevelName` true))
  (bind _output_get_2 (set `self.currentLevel` _returnvalue_2))
  (if (`KismetStringLibrary.EqualEqual_StrStr` _output_get_2 "JYPEscapeFloor")
    (bind _asgi_game_instance (cast `/Game/JYP/Blueprints/GI_GameInstance` (`GameplayStatics.GetGameInstance`)))
    (bind _previouslevel (`/Game/JYP/Blueprints/GI_GameInstance.previousLevel` _asgi_game_instance))
    (`KismetSystemLibrary.PrintString` _previouslevel)
    (bind (_lefts_2 _rights_2) (`KismetStringLibrary.Split` _previouslevel "_"))
    (`KismetSystemLibrary.PrintString` _rights_2)
    (bind (_value_2 _returnvalue_3) (`BlueprintMapLibrary.Map_Find` (`self.levelNameFilter`) _rights_2))
    (bind _returnvalue_4 (`PrimitiveComponent.CreateDynamicMaterialInstance` (`self.Plane`) 0 _value_2 "None"))
    (if _returnvalue_3
      (bind (_direction _appearance) (`Timeline|Timeline_0` :!via `PlayFromStart`)
        (:`Update`
          (`MaterialInstanceDynamic.SetScalarParameterValue` _returnvalue_4 "Opacity" _appearance))
        (:`Finished`
          (set `/Game/JYP/Blueprints/BP_JYPTestPlayer.bPlayerCanPressNextDoor?` true (`self.Player`)))))
    (else
      (`KismetSystemLibrary.PrintString` _rights)
      (if _returnvalue
        (bind _returnvalue_5 (`PrimitiveComponent.CreateDynamicMaterialInstance` (`self.Plane`) 0 _value "None"))
        (bind (_direction_2 _appearance_2) (`Timeline|CardAppearance` :!via `PlayFromStart`)
          (:`Update`
            (`MaterialInstanceDynamic.SetScalarParameterValue` _returnvalue_5 "Opacity" _appearance_2))
          (:`Finished`
            (set `/Game/JYP/Blueprints/BP_JYPTestPlayer.bPlayerCanPressNextDoor?` true (`self.Player`))))))))

(fn `UserConstructionScript`)