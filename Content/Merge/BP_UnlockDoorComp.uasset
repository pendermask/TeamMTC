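; Door-unlock component that moves the player through the MTower levels via one event per card, and handles the final restart or quit.
; Each event opens a hardcoded level by name, chaining Lobby, Normal, Grace, Life, Death and Magician, a stopgap for a planned map lookup.
; Both Opening events increment a shared card counter that gates loading the Lobby.
; BeginPlay caches the current level name, which is not used here.
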(event `self.ReceiveBeginPlay`
  ;[1 1 1] map으로 현재 레벨과 다음으로 가야 할 레벨 비교 및 제출한 카드를 확인해서 옮기는게 가장 좋을 거 같지만 우선 급한대로 각 카드에 사용될 함수들을 만들었음
  (bind _returnvalue (`GameplayStatics.GetCurrentLevelName` true))
  (set `self.currentLevel` _returnvalue))

(event `Unlock_Opening_Magician`
  (bind _returnvalue (+ (`self.checkCardCount`) 1))
  ;[1 1 1] map으로 현재 레벨과 다음으로 가야 할 레벨 비교 및 제출한 카드를 확인해서 옮기는게 가장 좋을 거 같지만 우선 급한대로 각 카드에 사용될 함수들을 만들었음
  (set `self.checkCardCount` _returnvalue)
  (if (<= _returnvalue 2)
    (`GameplayStatics.OpenLevel` "MTowerLobbyFloor_Lobby")))

(event `Unlock_Life`
  ;[1 1 1] map으로 현재 레벨과 다음으로 가야 할 레벨 비교 및 제출한 카드를 확인해서 옮기는게 가장 좋을 거 같지만 우선 급한대로 각 카드에 사용될 함수들을 만들었음
  (`GameplayStatics.OpenLevel` "MTowerFourthFloor_Death"))

(event `Unlock_Opening_Tower`
  (bind _returnvalue (+ (`self.checkCardCount`) 1))
  ;[1 1 1] map으로 현재 레벨과 다음으로 가야 할 레벨 비교 및 제출한 카드를 확인해서 옮기는게 가장 좋을 거 같지만 우선 급한대로 각 카드에 사용될 함수들을 만들었음
  (set `self.checkCardCount` _returnvalue)
  (if (<= _returnvalue 2)
    (`GameplayStatics.OpenLevel` "MTowerLobbyFloor_Lobby")))

(event `Unlock_Death`
  ;[1 1 1] map으로 현재 레벨과 다음으로 가야 할 레벨 비교 및 제출한 카드를 확인해서 옮기는게 가장 좋을 거 같지만 우선 급한대로 각 카드에 사용될 함수들을 만들었음
  (`GameplayStatics.OpenLevel` "MTowerLastFloor_Magician"))

(event `Unlock_Lobby`
  ;[1 1 1] map으로 현재 레벨과 다음으로 가야 할 레벨 비교 및 제출한 카드를 확인해서 옮기는게 가장 좋을 거 같지만 우선 급한대로 각 카드에 사용될 함수들을 만들었음
  (`GameplayStatics.OpenLevel` "MTowerFirstFloor_Normal"))

(event `Unlock_Magician_Restart`
  ;[1 1 1] map으로 현재 레벨과 다음으로 가야 할 레벨 비교 및 제출한 카드를 확인해서 옮기는게 가장 좋을 거 같지만 우선 급한대로 각 카드에 사용될 함수들을 만들었음
  (`GameplayStatics.OpenLevel` "MTowerLobbyFloor_Lobby"))

(event `Unlock_Normal`
  ;[1 1 1] map으로 현재 레벨과 다음으로 가야 할 레벨 비교 및 제출한 카드를 확인해서 옮기는게 가장 좋을 거 같지만 우선 급한대로 각 카드에 사용될 함수들을 만들었음
  (`GameplayStatics.OpenLevel` "MTowerSecondFloor_Grace"))

(event `Unlock_Magician_Escape`
  ;[1 1 1] map으로 현재 레벨과 다음으로 가야 할 레벨 비교 및 제출한 카드를 확인해서 옮기는게 가장 좋을 거 같지만 우선 급한대로 각 카드에 사용될 함수들을 만들었음
  (`KismetSystemLibrary.QuitGame` null "Quit"))

(event `Unlock_Grace`
  ;[1 1 1] map으로 현재 레벨과 다음으로 가야 할 레벨 비교 및 제출한 카드를 확인해서 옮기는게 가장 좋을 거 같지만 우선 급한대로 각 카드에 사용될 함수들을 만들었음
  (`GameplayStatics.OpenLevel` "MTowerThirdFloor_Life"))