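; BP_DefaultDeathMonster is a turn-based combat monster that fights the hand-tracking player.
; BeginPlay caches the game instance, player and BP_GMB game mode, then shows max health on its HP text.
; OnMyturn refreshes HP and, outside the player's turn, briefly shows any pending friendship dialogue from its friendship component.
; It then deals random damage through the player's health component, updates player HP text from the game instance and returns the turn via BP_GMB.
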(event `self.ReceiveBeginPlay`
  (bind _asgi_dgame_instance (cast `/Game/Merge/GI_DGameInstance` (`GameplayStatics.GetGameInstance`)))
  (set `self.GameInstance` _asgi_dgame_instance)
  (bind _asbp_default_hand_tracking_player (cast `/Game/Merge/BP_DefaultHandTrackingPlayer` (`GameplayStatics.GetPlayerPawn` 0)))
  (set `self.Player` _asbp_default_hand_tracking_player)
  (bind _asbp_gmb (cast `/Game/Merge/BP_GMB` (`GameplayStatics.GetGameMode`)))
  (set `self.GMB` _asbp_gmb)
  (`TextRenderComponent.K2_SetText` (`self.HP`) (`KismetTextLibrary.Conv_IntToText` (`/Game/Merge/BP_DefaultHealthComp.maxHealth` (`self.BP_DefaultHealthComp`)))))

(event `self.OnMyturn`
  (`TextRenderComponent.K2_SetText` (`self.HP`) (`KismetTextLibrary.Conv_IntToText` (`/Game/Merge/BP_DefaultHealthComp.currenthealth` (`self.BP_DefaultHealthComp`))))
  (if (not (`/Game/Merge/BP_DefaultHandTrackingPlayer.bPlayerTurn?` (`self.Player`)))
    (if (`/Game/Merge/BP_DefaultFriendshipComp.bMonsterGetFriendship?` (`self.BP_DefaultFriendshipComp`))
      (`SceneComponent.SetVisibility` (`self.TextRender`) true false)
      (`TextRenderComponent.K2_SetText` (`self.TextRender`) (`KismetTextLibrary.Conv_StringToText` (`/Game/Merge/BP_DefaultFriendshipComp.friendshipDialogueOutput` (`self.BP_DefaultFriendshipComp`))))
      (`KismetSystemLibrary.Delay` 3.0)
      (set `/Game/Merge/BP_DefaultFriendshipComp.bMonsterGetFriendship?` false (`self.BP_DefaultFriendshipComp`))
      (`SceneComponent.SetVisibility` (`self.TextRender`) false false))
    (bind _output_get (set `self.damage` (`KismetMathLibrary.RandomIntegerInRange` 1 7)))
    (`KismetSystemLibrary.Delay` 1.0)
    (`/Game/Merge/BP_DefaultHealthComp.Damaged` (`/Game/Merge/BP_DefaultHandTrackingPlayer.BP_DefaultHealthComp` (`self.Player`)) _output_get)
    (`KismetSystemLibrary.Delay` 2.0)
    (`TextRenderComponent.K2_SetText` (`/Game/Merge/BP_DefaultHandTrackingPlayer.HP` (`self.Player`)) (`KismetTextLibrary.Conv_IntToText` (`/Game/Merge/GI_DGameInstance.playerHealth` (`self.GameInstance`))))
    (`/Game/Merge/BP_GMB.PlayerTurn` (`self.GMB`))))

(fn `UserConstructionScript`)