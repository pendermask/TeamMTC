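; BP_DefaultLifeMonster is a Life-themed monster that takes turns against the hand-tracking player in a turn-based encounter with card-hit sounds.
; On BeginPlay it sets its health and friendship component sounds, caches game instance, player and game mode, and shows max HP.
; OnMyturn reacts to damage or friendship with timed Korean dialogue, then randomly attacks the player or, less often, heals itself.
; Delays pace the sequence before BP_GMB hands the turn back.
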(event `self.ReceiveBeginPlay`
  ;[1 1 1] Comment
  (set `/Game/Merge/BP_DefaultFriendshipComp.monsterGetFriendshipSound` "/Game/Asset/TTS/MonsterHit_TTS/Life/Life_lifecard_hit.Life_lifecard_hit" (`self.BP_DefaultFriendshipComp`))
  (set `/Game/Merge/BP_DefaultHealthComp.monsterDamagedSound` "/Game/Asset/TTS/MonsterHit_TTS/Life/Life_normalcard_hit.Life_normalcard_hit" (`self.BP_DefaultHealthComp`))
  (bind _asgi_dgame_instance (cast `/Game/Merge/GI_DGameInstance` (`GameplayStatics.GetGameInstance`)))
  (set `self.GameInstance` _asgi_dgame_instance)
  (bind _asbp_default_hand_tracking_player (cast `/Game/Merge/BP_DefaultHandTrackingPlayer` (`GameplayStatics.GetPlayerPawn` 0)))
  (set `self.Player` _asbp_default_hand_tracking_player)
  (bind _asbp_gmb (cast `/Game/Merge/BP_GMB` (`GameplayStatics.GetGameMode`)))
  (set `self.GMB` _asbp_gmb)
  (`TextRenderComponent.K2_SetText` (`self.HP`) (`KismetTextLibrary.Conv_IntToText` (`/Game/Merge/BP_DefaultHealthComp.maxHealth` (`self.BP_DefaultHealthComp`)))))

(event `self.OnMyturn`
  (set `self.randomForAction` (`KismetMathLibrary.RandomIntegerInRange` 0 5))
  (if (`/Game/Merge/BP_DefaultHealthComp.bMonsterDamaged?` (`self.BP_DefaultHealthComp`))
    (`TextRenderComponent.K2_SetText` (`self.HP`) (`KismetTextLibrary.Conv_IntToText` (`/Game/Merge/BP_DefaultHealthComp.currenthealth` (`self.BP_DefaultHealthComp`))))
    (`SceneComponent.SetVisibility` (`self.monsterDialogue`) true false)
    (`TextRenderComponent.K2_SetText` (`self.monsterDialogue`) (`KismetTextLibrary.Conv_StringToText` "아프잖아요!"))
    (set `/Game/Merge/BP_DefaultHealthComp.bMonsterDamaged?` false (`self.BP_DefaultHealthComp`))
    (`KismetSystemLibrary.Delay` 2.0)
    (`SceneComponent.SetVisibility` (`self.monsterDialogue`) true false))
  (if (not (`/Game/Merge/BP_DefaultHandTrackingPlayer.bPlayerTurn?` (`self.Player`)))
    (if (`/Game/Merge/BP_DefaultFriendshipComp.bMonsterGetFriendship?` (`self.BP_DefaultFriendshipComp`))
      (`SceneComponent.SetVisibility` (`self.monsterDialogue`) true false)
      (`TextRenderComponent.K2_SetText` (`self.monsterDialogue`) (`KismetTextLibrary.Conv_StringToText` (`/Game/Merge/BP_DefaultFriendshipComp.friendshipDialogueOutput` (`self.BP_DefaultFriendshipComp`))))
      (`KismetSystemLibrary.Delay` 2.0)
      (set `/Game/Merge/BP_DefaultFriendshipComp.bMonsterGetFriendship?` false (`self.BP_DefaultFriendshipComp`))
      (`SceneComponent.SetVisibility` (`self.monsterDialogue`) false false))
    (if (< (`self.randomForAction`) 4)
      (`SceneComponent.SetVisibility` (`self.monsterDialogue`) true false)
      (bind _output_get (set `self.damage` (`KismetMathLibrary.RandomIntegerInRange` 1 3)))
      (`KismetSystemLibrary.Delay` 1.0)
      (`/Game/Merge/BP_DefaultHealthComp.Damaged` (`/Game/Merge/BP_DefaultHandTrackingPlayer.BP_DefaultHealthComp` (`self.Player`)) _output_get)
      (`KismetSystemLibrary.Delay` 2.0)
      (`TextRenderComponent.K2_SetText` (`/Game/Merge/BP_DefaultHandTrackingPlayer.HP` (`self.Player`)) (`KismetTextLibrary.Conv_IntToText` (`/Game/Merge/GI_DGameInstance.playerHealth` (`self.GameInstance`))))
      (`TextRenderComponent.K2_SetText` (`self.monsterDialogue`) (`KismetTextLibrary.Conv_StringToText` "당신도 아프죠?"))
      (else
        (bind _output_get_2 (set `self.heal` (`KismetMathLibrary.RandomIntegerInRange` 1 3)))
        (`/Game/Merge/BP_DefaultHealthComp.Healing` (`self.BP_DefaultHealthComp`) _output_get_2)
        (`SceneComponent.SetVisibility` (`self.monsterDialogue`) true false)
        (`TextRenderComponent.K2_SetText` (`self.HP`) (`KismetTextLibrary.Conv_IntToText` (`/Game/Merge/BP_DefaultHealthComp.currenthealth` (`self.BP_DefaultHealthComp`))))
        (`TextRenderComponent.K2_SetText` (`self.monsterDialogue`) (`KismetTextLibrary.Conv_StringToText` (`KismetStringLibrary.Concat_StrStr` (`KismetStringLibrary.Conv_IntToString` (`self.heal`)) " 만큼 죽음과 멀어진다!")))))
    (`KismetSystemLibrary.Delay` 2.0)
    (`TextRenderComponent.K2_SetText` (`self.monsterDialogue`) (`KismetTextLibrary.Conv_StringToText` "후후, 다음엔 뭘 하실거죠?"))
    (`/Game/Merge/BP_GMB.PlayerTurn` (`self.GMB`))))

(fn `UserConstructionScript`)