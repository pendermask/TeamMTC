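; BP_DeathMonster is a monster in a turn-based fight against the BP_JYPTestPlayer character.
; On BeginPlay it caches the player and the BP_JYPGMB game mode.
; When OnMyturn fires outside the player's turn, it deals small random damage through the player's health component, prints debug messages and hands the turn back via the game mode.
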(event `self.ReceiveBeginPlay`
  (bind _asbp_jyptest_player (cast `/Game/JYP/Blueprints/BP_JYPTestPlayer` (`GameplayStatics.GetPlayerCharacter` 0)))
  (set `self.Player` _asbp_jyptest_player)
  (bind _asbp_jypgmb (cast `/Game/JYP/Blueprints/BP_JYPGMB` (`GameplayStatics.GetGameMode`)))
  (set `self.JYPGMB` _asbp_jypgmb))

(event `self.OnMyturn`
  (bind _player (`self.Player`))
  (if (not (`/Game/JYP/Blueprints/BP_JYPTestPlayer.bPlayerTurn?` _player))
    (bind _output_get (set `self.damage` (`KismetMathLibrary.RandomIntegerInRange` 1 3)))
    (`/Game/JYP/Blueprints/BP_HealthComp.Damaged` (`/Game/JYP/Blueprints/BP_JYPTestPlayer.BP_HealthComp` _player) _output_get)
    (`KismetSystemLibrary.PrintString` (`KismetStringLibrary.Concat_StrStr` "Attack : " (`KismetStringLibrary.Conv_IntToString` _output_get)))
    (`KismetSystemLibrary.PrintString` "Player Turn !")
    (`/Game/JYP/Blueprints/BP_JYPGMB.PlayerTurn` (`self.JYPGMB`))))

(fn `UserConstructionScript`)