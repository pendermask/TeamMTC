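; BP_GraceMonster is a monster in a turn-based exchange with the player that builds friendship on its turn.
; BeginPlay caches the game instance, the JYP test player and the JYP game mode.
; OnMyturn, outside the player's turn, raises FriendshipGrace by a small random amount and adds that whole running value, not just the increment, to TotalFriendship in the game instance.
; It then prints debug messages and calls PlayerTurn on the game mode.
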(event `self.ReceiveBeginPlay`
  ;[1 1 1] Comment
  (bind _asgi_game_instance (cast `/Game/JYP/Blueprints/GI_GameInstance` (`GameplayStatics.GetGameInstance`)))
  (set `self.GameInstance` _asgi_game_instance)
  (bind _asbp_jyptest_player (cast `/Game/JYP/Blueprints/BP_JYPTestPlayer` (`GameplayStatics.GetPlayerCharacter` 0)))
  (set `self.Player` _asbp_jyptest_player)
  (bind _asbp_jypgmb (cast `/Game/JYP/Blueprints/BP_JYPGMB` (`GameplayStatics.GetGameMode`)))
  (set `self.JYPGMB` _asbp_jypgmb))

(event `self.OnMyturn`
  (bind _gameinstance (`self.GameInstance`))
  ;[1 1 1] Comment
  (if (not (`/Game/JYP/Blueprints/BP_JYPTestPlayer.bPlayerTurn?` (`self.Player`)))
    (bind _output_get (set `self.friendship_Grace` (+ (`KismetMathLibrary.RandomIntegerInRange` 1 3) (`self.friendship_Grace`))))
    (set `/Game/JYP/Blueprints/GI_GameInstance.totalFriendship` (+ (`/Game/JYP/Blueprints/GI_GameInstance.totalFriendship` _gameinstance) _output_get) _gameinstance)
    (`KismetSystemLibrary.PrintString` (`KismetStringLibrary.Concat_StrStr` "My friendship is " (`KismetStringLibrary.Conv_IntToString` _output_get)))
    (`KismetSystemLibrary.PrintString` "Player Turn !")
    (`/Game/JYP/Blueprints/BP_JYPGMB.PlayerTurn` (`self.JYPGMB`))))

(fn `UserConstructionScript`)