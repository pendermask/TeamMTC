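; Normal monster for a turn-based game with a hand-tracking player; on its turn it shows a line of dialogue and passes play back.
; BeginPlay caches the player pawn and the BP_GMB game mode.
; OnMyturn, outside the player's turn, increments a counter to look up dialogue, falling back to final text, or shows dying text at low health.
; It then calls PlayerTurn on the game mode, with no attack logic.
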(event `self.ReceiveBeginPlay`
  ;[1 1 1] Caching
  (bind _asbp_default_hand_tracking_player (cast `/Game/Merge/BP_DefaultHandTrackingPlayer` (`GameplayStatics.GetPlayerPawn` 0)))
  (set `self.Player` _asbp_default_hand_tracking_player)
  (bind _asbp_gmb (cast `/Game/Merge/BP_GMB` (`GameplayStatics.GetGameMode`)))
  (set `self.GMB` _asbp_gmb))

(event `self.OnMyturn`
  ;[1 1 1] Comment
  (if (not (`/Game/Merge/BP_DefaultHandTrackingPlayer.bPlayerTurn?` (`self.Player`)))
    (bind _output_get (set `self.count` (+ (`self.count`) 1)))
    (if (<= (`/Game/Merge/BP_DefaultHealthComp.currenthealth` (`self.BP_DefaultHealthComp`)) 5)
      (`TextRenderComponent.K2_SetText` (`self.TextRender`) (`self.whenDying`))
      (else
        (bind (_value _returnvalue) (`BlueprintMapLibrary.Map_Find` (`self.Dialogue`) _output_get))
        (if _returnvalue
          (`TextRenderComponent.K2_SetText` (`self.TextRender`) _value)
          (else
            (`TextRenderComponent.K2_SetText` (`self.TextRender`) (`self.finalText`))))))
    (`KismetSystemLibrary.PrintString` "Player Turn !")
    (`/Game/Merge/BP_GMB.PlayerTurn` (`self.GMB`))))

(fn `UserConstructionScript`)