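; BP_Magician is a character that recaps the player's run through text-render dialogue and ends by awarding a composed title.
; BeginPlay caches the GameInstance and builds stat-based lines for kills, friendship, attribute card usage and choices.
; Each startDialogue call advances the line; after the last, setTitle joins threshold-picked fragments and a type lookup.
; The attribute tie check compares the value array with itself, so HighestType resolves to "Normal".
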(event `self.ReceiveBeginPlay`
  (bind _comparetypevalue (`self.compareTypeValue`))
  (bind _gameinstance (`self.GameInstance`))
  (bind _comparetypevalue_2 (`self.compareTypeValue`))
  (bind _dialogue (`self.dialogue`))
  (`|ExecutionSequence`
    (:`then_0`
      ;[1 1 1] Caching
      (bind _asgi_game_instance (cast `/Game/JYP/Blueprints/GI_GameInstance` (`GameplayStatics.GetGameInstance`)))
      (set `self.GameInstance` _asgi_game_instance)
      (`self.startDialogue`))
    (:`then_1`
      (`BlueprintMapLibrary.Map_Add` _comparetypevalue_2 "Normal" (`/Game/JYP/Blueprints/GI_GameInstance.normalValue` _gameinstance))
      (`BlueprintMapLibrary.Map_Add` _comparetypevalue_2 "Grace" (`/Game/JYP/Blueprints/GI_GameInstance.graceValue` _gameinstance))
      (`BlueprintMapLibrary.Map_Add` _comparetypevalue_2 "Life" (`/Game/JYP/Blueprints/GI_GameInstance.lifeValue` _gameinstance))
      (`BlueprintMapLibrary.Map_Add` _comparetypevalue_2 "Death" (`/Game/JYP/Blueprints/GI_GameInstance.deathValue` _gameinstance)))
    (:`then_2`
      ;[1 1 1] Set dialogue map
      (`BlueprintMapLibrary.Map_Add` _dialogue 5 (`KismetStringLibrary.Concat_StrStr` "You sacrificed " (`KismetStringLibrary.Conv_IntToString` (`/Game/JYP/Blueprints/GI_GameInstance.deadMonsterCount` (`self.GameInstance`))) " monsters to get up here."))
      (bind _values (`BlueprintMapLibrary.Map_Values` _comparetypevalue))
      (bind _keys (`BlueprintMapLibrary.Map_Keys` _comparetypevalue))
      (if (`KismetArrayLibrary.Array_Identical` _values _values)
        (set `self.highestType` "Normal")
        (else
          (bind _returnvalue (`KismetStringLibrary.Concat_StrStr` "You used the " (`|GetArrayItem` _keys (`KismetMathLibrary.MaxOfIntArray` _values)) " attribute card the most until you came up here..."))
          (set `self.highestType` _returnvalue)))
      (`BlueprintMapLibrary.Map_Add` _dialogue 7 _returnvalue)
      (`BlueprintMapLibrary.Map_Add` _dialogue 9 (`KismetStringLibrary.Concat_StrStr` "You've come this far with " (`KismetStringLibrary.Conv_IntToString` (`/Game/JYP/Blueprints/GI_GameInstance.playerActionCount` (`self.GameInstance`))) " choices."))
      (if (< (`/Game/JYP/Blueprints/GI_GameInstance.totalFriendship` (`self.GameInstance`)) 5)
        (`BlueprintMapLibrary.Map_Add` _dialogue 6 "You're quite liked by the monsters.")
        (else
          (`BlueprintMapLibrary.Map_Add` _dialogue 6 "Well, you're emotionally dry."))))))

(event `setTitle`
  (bind (_value _returnvalue) (`BlueprintMapLibrary.Map_Find` (`self.typeString`) (`self.highestType`)))
  (`|ExecutionSequence`
    (:`then_0`
      (if (> (`/Game/JYP/Blueprints/GI_GameInstance.deadMonsterCount` (`self.GameInstance`)) 2)
        (set `self.title_kill` "aggressive but, ")
        (else
          (set `self.title_kill` "chicken but, "))))
    (:`then_1`
      (if (> (`/Game/JYP/Blueprints/GI_GameInstance.totalFriendship` (`self.GameInstance`)) 3)
        (set `self.title_friendship` "warmly ")
        (else
          (set `self.title_friendship` "cold-hearted "))))
    (:`then_2`
      (if _returnvalue
        (set `self.title_type` (`KismetStringLibrary.Concat_StrStr` _value " "))))
    (:`then_3`
      (if (> (`/Game/JYP/Blueprints/GI_GameInstance.playerActionCount` (`self.GameInstance`)) 5)
        (set `self.title_actionCount` "game addict")
        (else
          (set `self.title_actionCount` "game hater"))))))

(event `startDialogue`
  (bind _textrender (`self.TextRender`))
  (bind (_value _returnvalue) (`BlueprintMapLibrary.Map_Find` (`self.dialogue`) (`self.dialogueIndex`)))
  (bind _returnvalue_2 (`KismetTextLibrary.Conv_StringToText` (`KismetStringLibrary.Concat_StrStr` (`self.title_kill`) (`self.title_friendship`) (`self.title_type`) (`self.title_actionCount`))))
  ;[1 1 1] Dialogue
  (if (< (`self.dialogueIndex`) 10)
    (set `self.dialogueIndex` (+ (`self.dialogueIndex`) 1))
    (if _returnvalue
      (`TextRenderComponent.K2_SetText` (`self.TextRender`) (`KismetTextLibrary.Conv_StringToText` _value)))
    (else
      (`self.setTitle`)
      (`TextRenderComponent.SetTextRenderColor` _textrender (`self.titleTextColor`))
      (`TextRenderComponent.K2_SetText` _textrender _returnvalue_2)
      (`KismetSystemLibrary.PrintString` (`KismetTextLibrary.Conv_TextToString` _returnvalue_2)))))

(fn `UserConstructionScript`)