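; BP_DefaultGraceMonster is a turn-based monster whose turn builds friendship.
; On BeginPlay it caches the game instance, hand-tracking player pawn and BP_GMB game mode.
; OnMyturn, when it is not the player's turn, randomly increases FriendshipGrace, adds that running value to the game instance's TotalFriendship, prints status, then returns the turn through the game mode.
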(event `self.ReceiveBeginPlay`
  ;[1 1 1] Comment
  (bind _asgi_dgame_instance (cast `/Game/Merge/GI_DGameInstance` (`GameplayStatics.GetGameInstance`)))
  (set `self.GameInstance` _asgi_dgame_instance)
  (bind _asbp_default_hand_tracking_player (cast `/Game/Merge/BP_DefaultHandTrackingPlayer` (`GameplayStatics.GetPlayerPawn` 0)))
  (set `self.Player` _asbp_default_hand_tracking_player)
  (bind _asbp_gmb (cast `/Game/Merge/BP_GMB` (`GameplayStatics.GetGameMode`)))
  (set `self.GMB` _asbp_gmb))

(event `self.OnMyturn`
  (bind _gameinstance (`self.GameInstance`))
  ;[1 1 1] Comment
  (if (not (`/Game/Merge/BP_DefaultHandTrackingPlayer.bPlayerTurn?` (`self.Player`)))
    (bind _output_get (set `self.friendship_Grace` (+ (`KismetMathLibrary.RandomIntegerInRange` 1 3) (`self.friendship_Grace`))))
    (set `/Game/Merge/GI_DGameInstance.totalFriendship` (+ (`/Game/Merge/GI_DGameInstance.totalFriendship` _gameinstance) _output_get) _gameinstance)
    (`KismetSystemLibrary.PrintString` (`KismetStringLibrary.Concat_StrStr` "My friendship is " (`KismetStringLibrary.Conv_IntToString` _output_get)))
    (`KismetSystemLibrary.PrintString` "Player Turn !")
    (`/Game/Merge/BP_GMB.PlayerTurn` (`self.GMB`))))

(fn `UserConstructionScript`)