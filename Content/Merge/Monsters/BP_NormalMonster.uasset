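; BP_NormalMonster is a turn-based monster that speaks a line of dialogue on its turn, then passes play back to the player.
; BeginPlay caches the BP_JYPTestPlayer character and the BP_JYPGMB game mode.
; OnMyturn, outside the player's turn, increments a counter and shows the matching Dialogue map entry, a fallback line, or a dying line at low health.
; It takes no attack action before calling PlayerTurn on the game mode.
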(event `self.ReceiveBeginPlay`
  (bind _asbp_jyptest_player (cast `/Game/JYP/Blueprints/BP_JYPTestPlayer` (`GameplayStatics.GetPlayerCharacter` 0)))
  (set `self.Player` _asbp_jyptest_player)
  (bind _asbp_jypgmb (cast `/Game/JYP/Blueprints/BP_JYPGMB` (`GameplayStatics.GetGameMode`)))
  (set `self.JYPGMB` _asbp_jypgmb))

(event `self.OnMyturn`
  (if (not (`/Game/JYP/Blueprints/BP_JYPTestPlayer.bPlayerTurn?` (`self.Player`)))
    (bind _output_get (set `self.count` (+ (`self.count`) 1)))
    (if (<= (`/Game/JYP/Blueprints/BP_HealthComp.currenthealth` (`self.BP_HealthComp`)) 5)
      (`TextRenderComponent.K2_SetText` (`self.TextRender`) (`self.whenDying`))
      (else
        (bind (_value _returnvalue) (`BlueprintMapLibrary.Map_Find` (`self.Dialogue`) _output_get))
        (if _returnvalue
          (`TextRenderComponent.K2_SetText` (`self.TextRender`) _value)
          (else
            (`TextRenderComponent.K2_SetText` (`self.TextRender`) (`self.finalText`))))))
    (`KismetSystemLibrary.PrintString` "Player Turn !")
    (`/Game/JYP/Blueprints/BP_JYPGMB.PlayerTurn` (`self.JYPGMB`))))

(fn `UserConstructionScript`)