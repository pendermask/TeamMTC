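; BP_DefaultQuitDoor is a door for the hand-tracking player that quits the game after a confirmation.
; On BeginPlay it shows its meshes, drives the Opacity of a Magician dynamic material on the plane with a timeline, then clears the player's PlayerCanPressNextDoor flag.
; The first Quit call changes the text to "Really?" and a second call quits.
; Nothing in this graph triggers Quit.
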(event `Quit`
  (bind _indexnumber (`self.indexNumber`))
  (if (< _indexnumber 1)
    (set `self.indexNumber` (+ _indexnumber 1))
    (`TextRenderComponent.K2_SetText` (`self.TextRender`) (`KismetTextLibrary.Conv_StringToText` "Really?"))
    (else
      (`KismetSystemLibrary.QuitGame` null "Quit"))))

(event `self.ReceiveBeginPlay`
  (bind _asbp_default_hand_tracking_player (cast `/Game/Merge/BP_DefaultHandTrackingPlayer` (`GameplayStatics.GetPlayerPawn` 0)))
  (set `self.Player` _asbp_default_hand_tracking_player)
  (`SceneComponent.SetVisibility` (`self.StaticMesh`) true false)
  (`SceneComponent.SetVisibility` (`self.Plane`) true false)
  (bind _returnvalue (`PrimitiveComponent.CreateDynamicMaterialInstance` (`self.Plane`) 0 "/Game/Asset/Cards/Grace/01_TheMagician_Mat.01_TheMagician_Mat" "None"))
  (bind (_direction _appearance) (`Timeline|Timeline_0` :!via `PlayFromStart`)
    (:`Update`
      (`MaterialInstanceDynamic.SetScalarParameterValue` _returnvalue "Opacity" _appearance))
    (:`Finished`
      (set `/Game/Merge/BP_DefaultHandTrackingPlayer.bPlayerCanPressNextDoor?` false (`self.Player`)))))

(fn `UserConstructionScript`)