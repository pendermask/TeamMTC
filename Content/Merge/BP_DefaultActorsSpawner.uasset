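; Level-placed spawner that fills its child actor components on BeginPlay according to the current level name.
; The name's suffix after the underscore keys a map for the monster or magician class, registered as CurrentEnemy on BP_JYPGMB; unmatched levels get a teleport door.
; The Magician last-floor level also gets restart and quit actors.
; An unconnected branch retains random monster selection from per-level index lists.
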(event `self.ReceiveBeginPlay`
  (bind _monsterormagician (`self.MonsterOrMagician`))
  (bind _returnvalue (`GameplayStatics.GetCurrentLevelName` true))
  (`|ExecutionSequence`
    (:`then_0`
      (bind (_value _returnvalue_2) (`BlueprintMapLibrary.Map_Find` (`self.spawnMonsterAndMagician`) (`.RightS` (`KismetStringLibrary.Split` _returnvalue "_"))))
      (if _returnvalue_2
        (`ChildActorComponent.SetChildActorClass` _monsterormagician _value)
        (bind _asbp_jypgmb (cast `/Game/JYP/Blueprints/BP_JYPGMB` (`GameplayStatics.GetGameMode`)))
        (set `/Game/JYP/Blueprints/BP_JYPGMB.currentEnemy` (`self.MonsterOrMagician`) _asbp_jypgmb)
        (else
          (`ChildActorComponent.SetChildActorClass` _monsterormagician "/Game/JYP/Blueprints/BP_TeleportDoor.BP_TeleportDoor_C"))))
    (:`then_1`
      (if (`KismetStringLibrary.EqualEqual_StrStr` _returnvalue "JYPTowerLastFloor_Magician")
        (`ChildActorComponent.SetChildActorClass` (`self.Restart`) "/Game/JYP/Blueprints/BP_Restart.BP_Restart_C")
        (`ChildActorComponent.SetChildActorClass` (`self.End`) "/Game/JYP/Blueprints/BP_Quit.BP_Quit_C")))))

(fn `UserConstructionScript`)