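; Highlight component that draws a colored outline around its owner's static mesh when OnOutline fires and Interactable is true.
; It spawns a collision-free copy of that mesh at the same transform, scaled by Thickness, with a dynamic MAT_Outline instance on slot 0 taking OutlineColor and Thickness.
; Each copy lives only 0.1 seconds, so the outline lasts only while OnOutline keeps being called.
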(event `OnOutline`
  (if (`self.bInteractable?`)
    (bind (_componentclass _spawnactorstaticmesh) (`self.CheckComponent`))
    (`StaticMeshActor.SetMobility` _spawnactorstaticmesh "Movable")
    (`Actor.SetLifeSpan` _spawnactorstaticmesh 0.1)
    (`Actor.SetActorEnableCollision` _spawnactorstaticmesh false)
    (bind _staticmeshcomponent (`StaticMeshActor.StaticMeshComponent` _spawnactorstaticmesh))
    (`StaticMeshComponent.SetStaticMesh` _staticmeshcomponent (`StaticMeshComponent.StaticMesh` _componentclass))
    (`SceneComponent.SetVisibility` _staticmeshcomponent true false)
    (bind _returnvalue (`PrimitiveComponent.CreateDynamicMaterialInstance` _staticmeshcomponent 0 "/Game/JYP/Assets/Material/MAT_Outline.MAT_Outline" "None"))
    (`MaterialInstanceDynamic.SetVectorParameterValue` _returnvalue "color" (`self.outlineColor`))
    (`MaterialInstanceDynamic.SetScalarParameterValue` _returnvalue "thickness" (`self.thickness`))))

(fn `CheckComponent`
  (returns (ComponentClass :type "StaticMeshComponent Object Reference") (SpawnActorStaticMesh :type "StaticMeshActor Object Reference"))
  (bind _returnvalue (`Actor.GetComponentByClass` (`self.GetOwner`) "/Script/Engine.StaticMeshComponent"))
  (bind (_returnvalue_location _returnvalue_rotation _returnvalue_scale) (`KismetMathLibrary.BreakTransform` (`SceneComponent.K2_GetComponentToWorld` _returnvalue)))
  (bind _returnvalue_2 (`|SpawnActorFromClass` "/Script/Engine.StaticMeshActor" (`KismetMathLibrary.MakeTransform` _returnvalue_location _returnvalue_rotation (* _returnvalue_scale (`self.thickness`))) "Undefined" "OverrideRootScale" null null))
  (return _returnvalue _returnvalue_2))