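; Hand-tracked VR player pawn for a card game, letting the player open a hand of cards, grab one and shoot it.
; Gesture events spawn a card spawner above the left palm, attach a grabbed card to the right palm, or cancel it.
; Shooting adds a name-matched particle, moves the card toward the actors spawner, triggers its action and notifies the GameMode.
; Tick sphere-traces from the camera for highlights, gaze-timed letters, monsters, cards and restart.
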(event `Left_Interaction`
  ;[1 1 1] Comment
  (bind _output_get (set `self.L_Interaction` true))
  (if (stale `Right_Interaction` _output_get)
    (`self.Interaction`)))

(event `Right_Interaction`
  ;[1 1 1] Comment
  (bind _output_get (set `self.R_Interaction` true))
  (if (stale `Left_Interaction` _output_get)
    (`self.Interaction`)))

(event `PlayerTurnEnd`
  ;[1 1 1] 플레이어의 패가 다 사라져야 함
  (`KismetSystemLibrary.Delay` 2.0)
  (`self.CardsOff`))

(event `Interaction`
  ;[1 1 1] Comment
  (`KismetSystemLibrary.PrintString` "Hello"))

(event `ShootCard`
  (bind _grabbedcard (`self.GrabbedCard`))
  (bind _grabbedcard_2 (`self.GrabbedCard`))
  (bind (_value _returnvalue) (`BlueprintMapLibrary.Map_Find` (`self.Particles`) (`KismetStringLibrary.Split` (`KismetSystemLibrary.GetDisplayName` (`self.GrabbedCard`)) "-")))
  ;[0 0 0 0 50] ShootCard
  (if (`self.GrabOn?`)
    (set `self.ShootCard?` true)
    (bind _returnvalue_2 (`GameplayStatics.GetActorOfClass` "/Game/Merge/BP_DefaultActorsSpawner.BP_DefaultActorsSpawner_C"))
    (if _returnvalue
      (`GameplayStatics.SpawnEmitterAttached` _value (`Actor.RootComponent` (`self.GrabbedCard`)) "None" (0.0 0.0 0.0) (struct) (0.5 0.5 0.5))
      (set `self.makeTransform` (`self.GetTransform` (`self.GetParentActor` (`self.GrabbedCard`))))
      (bind _asbp_dcard_parents (cast `/Game/Merge/Cards/BP_DCardParents` (`self.GrabbedCard`)))
      (bind _asbp_gmb (cast `/Game/Merge/BP_GMB` (`GameplayStatics.GetGameMode`)))
      (`/Game/Merge/BP_GMB.PlayerShot` _asbp_gmb)
      (`KismetSystemLibrary.MoveComponentTo` (`Actor.RootComponent` (`self.GrabbedCard`)) (`KismetMathLibrary.InverseTransformLocation` (`self.makeTransform`) (+ (`self.K2_GetActorLocation` _returnvalue_2) (0.0 0.0 150.0))) (`KismetMathLibrary.MakeRotFromY` (`self.GetActorRightVector` (`self.GrabbedCard`))) false false 1.0 true)
      (`/Engine/EditorBlueprintResources/StandardMacros.IsValid` _asbp_dcard_parents
        (:`Is Valid`
          (`/Game/Merge/Cards/BP_DCardParents.CardAction` _asbp_dcard_parents)
          (set `self.GrabOn?` false)
          (set `self.ShootCard?` false)
          (`GameplayStatics.GetCurrentLevelName` true)
          (if (`self.bPlayerCanPressNextDoor?`)
            (`/Engine/EditorBlueprintResources/StandardMacros.IsValid` _grabbedcard_2
              (:`Is Valid`
                (`self.K2_DestroyActor` _grabbedcard_2)))
            (else
              ;;[1 1 1] Comment
              (set `self.bPlayerTurn?` false)
              (set `self.bPlayerCanCardOpen?` false)
              (`/Engine/EditorBlueprintResources/StandardMacros.IsValid` _grabbedcard
                (:`Is Valid`
                  (`self.K2_DestroyActor` _grabbedcard)))))))
      (else
        (`KismetSystemLibrary.PrintString` "EMITTER ERROR")))))

(event `Key|P`
  (params (Key :type "Key Structure"))
  ;[1 1 1 0] save gesture, not use when player in game.
  (:`Pressed`
    (`HTHandTrackingGestureComponent.SaveGesture` (`self.HTHandTrackingGesture`) "/Game/HOO/Gesture/RHG_Interaction.RHG_Interaction" "Right" false (-1.0 -1.0 -1.0))
    (`KismetSystemLibrary.PrintString` "Saved")))

(event `Initialize`
  ;[1 1 1] Comment
  ;;[1 1 1] Comment
  (if (`self.bPlayerTurn?`)
    (if (not (`self.GrabOn?`)) :!label _label
      (set `self.InitializeCards` true)
      (if (`self.PlayStart`)
        (`/Engine/EditorBlueprintResources/StandardMacros.IsValid` (`self.CardSpawner`)
          (:`Is Valid`
            (`self.K2_DestroyActor` (`self.CardSpawner`)))))
      (set `self.CardsOn?` false))
    (elif (`self.bPlayerCanCardOpen?`)
      (goto _label))))

(event `self.ReceiveBeginPlay`
  ;[1 1 1] Comment
  (`HeadMountedDisplayFunctionLibrary.SetTrackingOrigin` "Floor"))

(event `CardsOn`
  (bind (_returnvalue_x _returnvalue_y _returnvalue_z) (`KismetMathLibrary.BreakVector` (`HandTrackingFL.GetHandPalmLocation` (`self.LeftHandTracking`))))
  (bind _returnvalue (`KismetMathLibrary.MakeVector` _returnvalue_x _returnvalue_y (+ _returnvalue_z 20.0)))
  (bind (_returnvalue_roll _returnvalue_pitch _returnvalue_yaw) (`KismetMathLibrary.BreakRotator` (`KismetMathLibrary.Conv_VectorToRotator` (- _returnvalue (`SceneComponent.K2_GetComponentLocation` (`self.Camera`))))))
  ;[1 1 1] Comment
  (if (`self.CardsOn?`)
    _
    (elif (`self.InitializeCards`)
      (bind _returnvalue_2 (`|SpawnActorFromClass` "/Game/Merge/BP_DefaultHandCardSpawner.BP_DefaultHandCardSpawner_C" (`KismetMathLibrary.MakeTransform` _returnvalue (`KismetMathLibrary.MakeRotator` _returnvalue_roll 0.0 (+ _returnvalue_yaw 90.0))) "Undefined" "OverrideRootScale" null null))
      (set `self.CardSpawner` _returnvalue_2)
      (set `self.PlayStart` true)
      (set `self.CardsOn?` true)
      (set `self.InitializeCards` false))))

(event `self.ReceiveTick`
  (params (DeltaSeconds :type "Float (single-precision)"))
  (bind _grabbedcard (`self.GrabbedCard`))
  (bind (_returnvalue_x _returnvalue_y _returnvalue_z) (`KismetMathLibrary.BreakVector` (`HandTrackingFL.GetHandPalmLocation` (`self.RightHandTracking`))))
  (bind _transformcomponent (`PlayerCameraManager.TransformComponent` (`GameplayStatics.GetPlayerCameraManager` 0)))
  (bind _returnvalue (`SceneComponent.K2_GetComponentLocation` _transformcomponent))
  (bind _returnvalue_2 (`KismetMathLibrary.MakeVector` _returnvalue_x _returnvalue_y (+ _returnvalue_z 20.0)))
  (bind (_returnvalue_roll _returnvalue_pitch _returnvalue_yaw) (`KismetMathLibrary.BreakRotator` (`KismetMathLibrary.Conv_VectorToRotator` (- _returnvalue_2 (`SceneComponent.K2_GetComponentLocation` (`self.Camera`))))))
  ;[1 1 1] Comment
  (`|ExecutionSequence`
    (:`then_0`
      (if (and (`self.GrabOn?`) (not (`self.ShootCard?`)))
        (`/Engine/EditorBlueprintResources/StandardMacros.IsValid` _grabbedcard
          (:`Is Valid`
            (`self.K2_SetActorTransform` _grabbedcard (`KismetMathLibrary.MakeTransform` _returnvalue_2 (`KismetMathLibrary.MakeRotator` _returnvalue_roll 0.0 (+ _returnvalue_yaw 90.0))) false false)))))
    (:`then_1`
      ;[1 1 1] Comment
      (bind (_outhit _returnvalue_3) (`KismetSystemLibrary.SphereTraceSingleForObjects` :`Start` _returnvalue :`End` (+ (* (`SceneComponent.GetForwardVector` _transformcomponent) 1000.0) _returnvalue) :`Radius` 10.0 :`ObjectTypes` (`self.PlayerTrackingObjectTypes`) :`DrawDebugType` "ForOneFrame"))
      (if _returnvalue_3
        (`|ExecutionSequence`
          (:`then_0`
            (bind (_bblockinghit _binitialoverlap _time _distance _location _impactpoint _normal _impactnormal _physmat _hitactor _hitcomponent) (`GameplayStatics.BreakHitResult` _outhit))
            (bind _returnvalue_4 (`self.GetComponentByClass` _hitactor "/Game/Merge/BP_DefaultHighlightComp.BP_DefaultHighlightComp_C"))
            (`/Engine/EditorBlueprintResources/StandardMacros.IsValid` _returnvalue_4
              (:`Is Valid`
                (`/Game/Merge/BP_DefaultHighlightComp.OnOutline` _returnvalue_4))))
          (:`then_1`
            (bind _asbp_default_letter (cast `/Game/Merge/BP_DefaultLetter` _hitactor))
            (set `self.bLetterHere?` true)
            (set `self.Letter` _asbp_default_letter)
            (set `self.currentLetterWatchingTime` (+ (`self.currentLetterWatchingTime`) DeltaSeconds))
            (if (<= (`self.letterInteractionTime`) (`self.currentLetterWatchingTime`))
              (`/Game/Merge/BP_DefaultLetter.WhenClickLetter` (`self.Letter`))
              (set `self.bLetterTextHere?` true)))
          (:`then_2`
            (cast `/Game/JYP/Blueprints/Monster/BP_MonsterParent` _hitactor
              (:`then`
                (set `self.bPlayerSeeMonster?` true))
              (:`CastFailed`
                (set `self.bPlayerSeeMonster?` false))))
          (:`then_3`
            (bind _asbp_restart (cast `/Game/JYP/Blueprints/BP_Restart` _hitactor))
            (set `self.Restart` _asbp_restart)
            (set `self.bPlayerSeeRestart?` true))
          (:`then_4`
            (cast `/Game/Merge/Cards/BP_DCardParents` _hitactor
              (:`then`
                (set `self.bPlayerSeeCard?` true))
              (:`CastFailed`
                (set `self.bPlayerSeeCard?` false)))))
        (else
          (set `self.bLetterHere?` false)
          (set `self.bPlayerSeeRestart?` false)
          (set `self.currentLetterWatchingTime` 0.0)
          (set `self.bPlayerSeeCard?` false))))))

(event `Key|RightMouseButton`
  (params (Key :type "Key Structure"))
  ;[1 1 1] Comment
)

(event `CardsOff`
  ;[1 1 1] Comment
  (if (`self.CardsOn?`)
    (`/Engine/EditorBlueprintResources/StandardMacros.IsValid` (`self.CardSpawner`)
      (:`Is Valid`
        (`self.K2_DestroyActor` (`self.CardSpawner`))
        (set `self.CardsOn?` false)
        (set `self.GrabOn?` false)))))

(event `Grab1`
  ;[1 1 1] Comment
  (if (and (`self.CardsOn?`) (not (`self.GrabOn?`)))
    (set `self.GrabOn?` true)
    (bind _returnvalue (`GameplayStatics.GetActorOfClass` "/Game/Merge/BP_DefaultHandCardSpawner.BP_DefaultHandCardSpawner_C"))
    (bind _returnvalue_2 (`GameplayStatics.GetActorOfClass` (`ChildActorComponent.ChildActorClass` (`/Game/Merge/BP_DefaultHandCardSpawner.Child1` _returnvalue))))
    (set `self.GrabbedCard` _returnvalue_2)))

(event `Grab2`
  ;[1 1 1] Comment
  (if (and (`self.CardsOn?`) (not (`self.GrabOn?`)))
    (set `self.GrabOn?` true)
    (bind _returnvalue (`GameplayStatics.GetActorOfClass` "/Game/Merge/BP_DefaultHandCardSpawner.BP_DefaultHandCardSpawner_C"))
    (bind _returnvalue_2 (`GameplayStatics.GetActorOfClass` (`ChildActorComponent.ChildActorClass` (`/Game/Merge/BP_DefaultHandCardSpawner.Child2` _returnvalue))))
    (set `self.GrabbedCard` _returnvalue_2)))

(event `Grab3`
  ;[1 1 1] Comment
  (if (and (`self.CardsOn?`) (not (`self.GrabOn?`)))
    (set `self.GrabOn?` true)
    (bind _returnvalue (`GameplayStatics.GetActorOfClass` "/Game/Merge/BP_DefaultHandCardSpawner.BP_DefaultHandCardSpawner_C"))
    (bind _returnvalue_2 (`GameplayStatics.GetActorOfClass` (`ChildActorComponent.ChildActorClass` (`/Game/Merge/BP_DefaultHandCardSpawner.Child3` _returnvalue))))
    (set `self.GrabbedCard` _returnvalue_2)))

(event `Grab4`
  ;[1 1 1] Comment
  (if (and (`self.CardsOn?`) (not (`self.GrabOn?`)))
    (set `self.GrabOn?` true)
    (bind _returnvalue (`GameplayStatics.GetActorOfClass` "/Game/Merge/BP_DefaultHandCardSpawner.BP_DefaultHandCardSpawner_C"))
    (bind _returnvalue_2 (`GameplayStatics.GetActorOfClass` (`ChildActorComponent.ChildActorClass` (`/Game/Merge/BP_DefaultHandCardSpawner.Child4` _returnvalue))))
    (set `self.GrabbedCard` _returnvalue_2)))

(event `GrabCancel`
  (bind _grabbedcard (`self.GrabbedCard`))
  ;[1 1 1] Comment
  (if (`self.GrabOn?`)
    ;;[1 1 1] Comment
    (`/Engine/EditorBlueprintResources/StandardMacros.IsValid` _grabbedcard
      (:`Is Valid`
        (`self.K2_DestroyActor` _grabbedcard)
        (set `self.CardsOn?` false)
        (set `self.GrabOn?` false)))))

(fn `UserConstructionScript`)