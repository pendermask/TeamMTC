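; BP_DefaultRestartDoor is a door for the hand-tracking player that restarts the game by opening the tower lobby level.
; On BeginPlay it shows its mesh and plane, fades the plane in through a timeline-driven dynamic material, then lets the player press the next door.
; The Restart event uses a counter as confirmation: the first call displays a lost-records warning, and a later call loads the lobby.
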(event `Restart`
  (bind _indexnumber (`self.indexNumber`))
  (if (< _indexnumber 1)
    (set `self.indexNumber` (+ _indexnumber 1))
    (`TextRenderComponent.K2_SetText` (`self.TextRender`) (`KismetTextLibrary.Conv_StringToText` (`KismetStringLibrary.Concat_StrStr` "really? \n" "All your records will be lost.")))
    (else
      (`GameplayStatics.OpenLevel` "JYPTowerLobbyFloor_Lobby"))))

(event `self.ReceiveBeginPlay`
  (bind _asbp_default_hand_tracking_player (cast `/Game/Merge/BP_DefaultHandTrackingPlayer` (`GameplayStatics.GetPlayerPawn` 0)))
  (set `self.Player` _asbp_default_hand_tracking_player)
  (`SceneComponent.SetVisibility` (`self.StaticMesh`) true false)
  (`SceneComponent.SetVisibility` (`self.Plane`) true false)
  (bind _returnvalue (`PrimitiveComponent.CreateDynamicMaterialInstance` (`self.Plane`) 0 "/Game/Asset/Cards/Death/16_TheTower_Mat.16_TheTower_Mat" "None"))
  (bind (_direction _appearance) (`Timeline|Timeline_0` :!via `PlayFromStart`)
    (:`Update`
      (`MaterialInstanceDynamic.SetScalarParameterValue` _returnvalue "Opacity" _appearance))
    (:`Finished`
      (set `/Game/Merge/BP_DefaultHandTrackingPlayer.bPlayerCanPressNextDoor?` true (`self.Player`)))))

(fn `UserConstructionScript`)