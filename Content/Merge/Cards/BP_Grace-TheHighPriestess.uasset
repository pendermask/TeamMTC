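; Grace card "The High Priestess" for a hand-tracking player, acting as an attack against a monster.
; BeginPlay caches the player pawn and sets the card's type and value.
; Tick shows or hides a Cube tooltip according to the player's PlayerSeeCard flag.
; CardAction passes the card value as damage to the health component of the monster found by class, only while the player cannot press next door.
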(event `self.ReceiveTick`
  (params (DeltaSeconds :type "Float (single-precision)"))
  ;[1 1 1] Comment
  (if (`/Game/Merge/BP_DefaultHandTrackingPlayer.bPlayerSeeCard?` (`self.Player`))
    (`self.OnToolTip`)
    (else
      (`self.OffToolTip`))))

(event `self.ReceiveBeginPlay`
  ;[1 1 1] Comment
  (bind _asbp_default_hand_tracking_player (cast `/Game/Merge/BP_DefaultHandTrackingPlayer` (`GameplayStatics.GetPlayerPawn` 0)))
  (set `self.player` _asbp_default_hand_tracking_player)
  (set `self.cardTypeValue` 1)
  (set `self.cardType` "Grace"))

(event `self.OnToolTip`
  ;[1 1 1] Comment
  (`SceneComponent.SetVisibility` (`self.Cube`) true false))

(event `self.CardAction`
  (if (not (`/Game/Merge/BP_DefaultHandTrackingPlayer.bPlayerCanPressNextDoor?` (`self.Player`)))
    (bind _returnvalue (`GameplayStatics.GetActorOfClass` "/Game/Merge/Monsters/BP_DefaultMonsterParent.BP_DefaultMonsterParent_C"))
    (`/Game/Merge/BP_DefaultHealthComp.Damaged` (`self.GetComponentByClass` _returnvalue "/Game/Merge/BP_DefaultHealthComp.BP_DefaultHealthComp_C") (`self.cardTypeValue`))))

(event `self.OffToolTip`
  ;[1 1 1] Comment
  (`SceneComponent.SetVisibility` (`self.Cube`) false false))

(fn `UserConstructionScript`)