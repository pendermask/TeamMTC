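; The Magician Life card for a hand-tracking player, which either heals the player or unlocks a door when played.
; Tick shows or hides a tooltip cube based on the player's PlayerSeeCard flag.
; CardAction calls the unlock component's level-specific function, chosen by level name, when the player can press the next door.
; Otherwise it heals through the player's health component by the card's value.
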(event `self.ReceiveTick`
  (params (DeltaSeconds :type "Float (single-precision)"))
  ;[1 1 1] Comment
  (if (`/Game/Merge/BP_DefaultHandTrackingPlayer.bPlayerSeeCard?` (`self.Player`))
    (`self.OnToolTip`)
    (else
      (`self.OffToolTip`))))

(event `self.ReceiveBeginPlay`
  ;[1 1 1] Comment
  (bind _asbp_default_hand_tracking_player (cast `/Game/Merge/BP_DefaultHandTrackingPlayer` (`GameplayStatics.GetPlayerPawn` 0)))
  (set `self.player` _asbp_default_hand_tracking_player)
  (set `self.cardTypeValue` 1)
  (set `self.cardType` "Life"))

(event `self.OnToolTip`
  ;[1 1 1] Comment
  (`SceneComponent.SetVisibility` (`self.Cube`) true false))

(event `self.CardAction`
  (bind _bp_unlockdoorcomp (`self.BP_UnlockDoorComp`))
  (if (`/Game/Merge/BP_DefaultHandTrackingPlayer.bPlayerCanPressNextDoor?` (`self.Player`))
    (bind _returnvalue (`GameplayStatics.GetCurrentLevelName` true))
    (if (`KismetStringLibrary.EqualEqual_StrStr` _returnvalue "MOpening")
      (`/Game/Merge/BP_UnlockDoorComp.Unlock_Opening_Magician` _bp_unlockdoorcomp)
      (elif (`KismetStringLibrary.EqualEqual_StrStr` _returnvalue "MTowerFourthFloor_Death")
        (`/Game/Merge/BP_UnlockDoorComp.Unlock_Death` _bp_unlockdoorcomp)
        (else
          (`/Game/Merge/BP_UnlockDoorComp.Unlock_Magician_Escape` _bp_unlockdoorcomp))))
    (else
      (bind _returnvalue_2 (`GameplayStatics.GetActorOfClass` "/Game/Merge/BP_DefaultHandTrackingPlayer.BP_DefaultHandTrackingPlayer_C"))
      (`/Game/Merge/BP_DefaultHealthComp.Healing` (`self.GetComponentByClass` _returnvalue_2 "/Game/Merge/BP_DefaultHealthComp.BP_DefaultHealthComp_C") (`self.cardTypeValue`)))))

(event `self.OffToolTip`
  ;[1 1 1] Comment
  (`SceneComponent.SetVisibility` (`self.Cube`) false false))

(fn `UserConstructionScript`)