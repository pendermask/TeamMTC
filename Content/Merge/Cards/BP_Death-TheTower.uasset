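; BP_Death-TheTower is a card Blueprint of type "Death" that can unlock the tower opening.
; BeginPlay caches the hand-tracking player pawn and sets the card's value and type.
; Tick polls the player's PlayerSeeCard flag to show or hide a Cube component as the tooltip.
; CardAction calls UnlockOpeningTower on the unlock-door component when CardGame is off and PlayerCanCardOpen is set.
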(event `self.ReceiveTick`
  (params (DeltaSeconds :type "Float (single-precision)"))
  ;[1 1 1] Comment
  (if (`/Game/Merge/BP_DefaultHandTrackingPlayer.bPlayerSeeCard?` (`self.Player`))
    (`self.OnToolTip`)
    (else
      (`self.OffToolTip`))))

(event `self.ReceiveBeginPlay`
  ;[1 1 1] Comment
  (bind _asbp_default_hand_tracking_player (cast `/Game/Merge/BP_DefaultHandTrackingPlayer` (`GameplayStatics.GetPlayerPawn` 0)))
  (set `self.player` _asbp_default_hand_tracking_player)
  (set `self.Value` 3)
  (set `self.Type` "Death"))

(event `self.OnToolTip`
  ;[1 1 1] Comment
  (`SceneComponent.SetVisibility` (`self.Cube`) true false))

(event `self.OffToolTip`
  ;[1 1 1] Comment
  (`SceneComponent.SetVisibility` (`self.Cube`) false false))

(event `self.CardAction`
  (bind _player_0 (`self.Player_0`))
  ;[1 1 1] Comment
  (if (`/Game/Merge/BP_DefaultHandTrackingPlayer.bCardGame?` _player_0)
    _
    (elif (`/Game/Merge/BP_DefaultHandTrackingPlayer.bPlayerCanCardOpen?` _player_0)
      (`/Game/Merge/BP_UnlockDoorComp.Unlock_Opening_Tower` (`self.BP_UnlockDoorComp`)))))

(fn `UserConstructionScript`)