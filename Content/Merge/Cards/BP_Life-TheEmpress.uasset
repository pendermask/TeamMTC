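; BP_Life-TheEmpress is a tarot-style "Life" card for a hand-tracking player that heals when its action fires.
; BeginPlay caches the player and game instance and sets the card's type and value.
; CardAction, unless the player can press the next door, adds the value to the game instance's life total and heals through the player's health component.
; Tick polls the player's see-card flag to show or hide the tooltip.
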(event `self.ReceiveTick`
  (params (DeltaSeconds :type "Float (single-precision)"))
  ;[1 1 1] Comment
  (if (`/Game/Merge/BP_DefaultHandTrackingPlayer.bPlayerSeeCard?` (`self.Player`))
    (`self.OnToolTip`)
    (else
      (`self.OffToolTip`))))

(event `self.ReceiveBeginPlay`
  ;[1 1 1] Comment
  (bind _asbp_default_hand_tracking_player (cast `/Game/Merge/BP_DefaultHandTrackingPlayer` (`GameplayStatics.GetPlayerPawn` 0)))
  (set `self.player` _asbp_default_hand_tracking_player)
  (set `self.cardTypeValue` 2)
  (set `self.cardType` "Life")
  (bind _asgi_dgame_instance (cast `/Game/Merge/GI_DGameInstance` (`GameplayStatics.GetGameInstance`)))
  (set `self.gameInstance` _asgi_dgame_instance))

(event `self.OnToolTip`
  ;[1 1 1] Comment
  (`SceneComponent.SetVisibility` (`self.Tooltip`) true false))

(event `self.CardAction`
  (bind _gameinstance (`self.GameInstance`))
  (if (not (`/Game/Merge/BP_DefaultHandTrackingPlayer.bPlayerCanPressNextDoor?` (`self.Player`)))
    (set `/Game/Merge/GI_DGameInstance.lifeValue` (+ (`/Game/Merge/GI_DGameInstance.lifeValue` _gameinstance) (`self.cardTypeValue`)) _gameinstance)
    (bind _returnvalue (`GameplayStatics.GetActorOfClass` "/Game/Merge/BP_DefaultHandTrackingPlayer.BP_DefaultHandTrackingPlayer_C"))
    (`/Game/Merge/BP_DefaultHealthComp.Healing` (`self.GetComponentByClass` _returnvalue "/Game/Merge/BP_DefaultHealthComp.BP_DefaultHealthComp_C") (`self.cardTypeValue`))))

(event `self.OffToolTip`
  ;[1 1 1] Comment
  (`SceneComponent.SetVisibility` (`self.Tooltip`) false false))

(fn `UserConstructionScript`)