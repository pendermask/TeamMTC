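; Game manager for a hand-tracking card battle, running timed turns between the player and a monster.
; BeginPlay caches the game instance, player and current enemy's child-actor monster.
; CardGame either runs a timeline countdown on the player's turn, then counts the action and re-enters itself, or hands off to the monster's OnMyturn.
; External events restart player turns, rewind the timer on a shot, and spawn a teleport door.
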(event `SpawnTeleportDoor`
  (params (NewParam :type "Transform Structure"))
  ;[1 1 1] spawn door after monster dead
  (`|SpawnActorFromClass` "/Game/Merge/BP_DefaultTeleportDoor.BP_DefaultTeleportDoor_C" NewParam "Undefined" "OverrideRootScale" null null))

(event `self.ReceiveBeginPlay`
  (bind _currentenemy (`self.currentEnemy`))
  ;[1 1 1] Caching
  (bind _asgi_dgame_instance (cast `/Game/Merge/GI_DGameInstance` (`GameplayStatics.GetGameInstance`)))
  (set `self.GameInstance` _asgi_dgame_instance)
  (bind _asbp_default_hand_tracking_player (cast `/Game/Merge/BP_DefaultHandTrackingPlayer` (`GameplayStatics.GetPlayerPawn` 0)))
  (set `self.Player` _asbp_default_hand_tracking_player)
  (`/Engine/EditorBlueprintResources/StandardMacros.IsValid` _currentenemy
    (:`Is Valid`
      (set `/Game/Merge/BP_DefaultHandTrackingPlayer.bPlayerTurn?` true _asbp_default_hand_tracking_player)
      (bind _asbp_default_monster_parent (cast `/Game/Merge/Monsters/BP_DefaultMonsterParent` (`ChildActorComponent.ChildActor` _currentenemy)))
      (set `self.MonsterParent` _asbp_default_monster_parent))))

(event `CardGame`
  (bind _player (`self.Player`))
  (bind _player_2 (`self.Player`))
  (bind _gameinstance (`self.GameInstance`))
  (bind _player_3 (`self.Player`))
  ;[1 1 1] Turn
  (`SceneComponent.SetVisibility` (`/Game/Merge/BP_DefaultHandTrackingPlayer.TurnTimer` _player) true false)
  (`SceneComponent.SetVisibility` (`/Game/Merge/BP_DefaultHandTrackingPlayer.HP` _player) true false)
  (`/Engine/EditorBlueprintResources/StandardMacros.IsValid` (`self.MonsterParent`)
    (:`Is Valid`
      (set `/Game/Merge/BP_DefaultHandTrackingPlayer.bCardGame?` false (`self.Player`))
      ;;[1 1 1] Comment
      (if (`/Game/Merge/BP_DefaultHandTrackingPlayer.bPlayerTurn?` (`self.Player`))
        ;;[1 1 1] player turn sound
        (`GameplayStatics.PlaySound2D` "/Game/Asset/Sound/TurnOn/myTurn.myTurn" 20.0 1.0 0.0 null null)
        (`SceneComponent.SetVisibility` (`/Game/Merge/BP_DefaultHandTrackingPlayer.SpotLight` (`self.Player`)) true false)
        (bind (_direction _taketurntime) (`Timeline|Timeline_0` :`NewTime` 29.5 :!via `PlayFromStart` :!label _label)
          (:`Update`
            (`TextRenderComponent.K2_SetText` (`/Game/Merge/BP_DefaultHandTrackingPlayer.TurnTimer` (`self.Player`)) (`KismetTextLibrary.Conv_Int64ToText` (`KismetMathLibrary.FCeil64` _taketurntime))))
          (:`Finished`
            (`SceneComponent.SetVisibility` (`/Game/Merge/BP_DefaultHandTrackingPlayer.SpotLight` (`self.Player`)) false false)
            (`SceneComponent.SetVisibility` (`/Game/Merge/BP_DefaultHandTrackingPlayer.clock` _player_2) false false)
            (`TextRenderComponent.K2_SetText` (`/Game/Merge/BP_DefaultHandTrackingPlayer.TurnTimer` _player_2) (`KismetTextLibrary.Conv_StringToText` "done!"))
            (set `/Game/Merge/BP_DefaultHandTrackingPlayer.bPlayerTurn?` false _player_3)
            (`/Game/Merge/BP_DefaultHandTrackingPlayer.PlayerTurnEnd` _player_3)
            (bind _output_get (set `/Game/Merge/GI_DGameInstance.playerActionCount` (+ (`/Game/Merge/GI_DGameInstance.playerActionCount` _gameinstance) 1) _gameinstance))
            (`KismetSystemLibrary.Delay` 1.0)
            (`self.CardGame`)))
        (else
          (`/Game/Merge/Monsters/BP_DefaultMonsterParent.OnMyturn` (`self.MonsterParent`)))))))

(event `PlayerShot`
  ;[1 1 1] Turn
  (`/Game/Merge/BP_DefaultHandTrackingPlayer.PlayerTurnEnd` (`self.Player`))
  (goto _label :!via `SetNewTime`))

(event `PlayerTurn`
  ;[1 1 1] Comment
  (set `/Game/Merge/BP_DefaultHandTrackingPlayer.bPlayerTurn?` true (`self.Player`))
  (set `/Game/Merge/BP_DefaultHandTrackingPlayer.bPlayerCanCardOpen?` true (`self.Player`))
  (`self.CardGame`))

(fn `UserConstructionScript`)