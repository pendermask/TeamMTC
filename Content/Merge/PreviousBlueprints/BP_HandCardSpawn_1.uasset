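; Card hand spawner that deals four random cards into four child actor components on BeginPlay.
; RandomArray shuffles the integer Deck through repeated random pair swaps, never picking the last element.
; The first four entries are copied into Hand without removal, then the previous Save is appended to Deck and replaced by Hand.
; Each Hand value indexes CardShuffle to set the child actor class for its slot.
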(event `self.ReceiveBeginPlay`
  (bind _eachcard (`self.EachCard`))
  (`KismetArrayLibrary.Array_Add` _eachcard (`self.Child1`))
  (`KismetArrayLibrary.Array_Add` _eachcard (`self.Child2`))
  (`KismetArrayLibrary.Array_Add` _eachcard (`self.Child3`))
  (`KismetArrayLibrary.Array_Add` _eachcard (`self.Child4`))
  (`KismetArrayLibrary.Array_Clear` (`self.Hand`))
  (`self.RandomArray`)
  (for _index (range 4)
    (`KismetArrayLibrary.Array_Add` (`self.Hand`) (`|GetArrayItem` (`self.deck`) _index)))
  (`KismetArrayLibrary.Array_Append` (`self.deck`) (`self.save`))
  (set `self.save` (`self.Hand`))
  (for (_array_element _array_index) (`self.Hand`)
    (`ChildActorComponent.SetChildActorClass` (`|GetArrayItem` (`self.EachCard`) _array_index) (`|GetArrayItem` (`self.CardShuffle`) _array_element))))

(fn `RandomArray`
  (bind _deck (`self.deck`))
  (bind _deck_2 (`self.deck`))
  (for _ (range 61)
    (bind _output_get (set `self.tempIndexInt` (`KismetMathLibrary.RandomInteger` (- (`KismetArrayLibrary.Array_Length` _deck_2) 1))))
    (set `self.tempInt` (`|GetArrayItem` _deck_2 _output_get))
    (bind _output_get_2 (set `self.temp2indexint` (`KismetMathLibrary.RandomInteger` (- (`KismetArrayLibrary.Array_Length` _deck) 1))))
    (set `self.temp2int` (`|GetArrayItem` _deck _output_get_2))
    (`KismetArrayLibrary.Array_Set` (`self.deck`) (`self.temp2indexint`) (`self.tempInt`))
    (`KismetArrayLibrary.Array_Set` (`self.deck`) (`self.tempIndexInt`) (`self.temp2int`))))

(fn `UserConstructionScript`)