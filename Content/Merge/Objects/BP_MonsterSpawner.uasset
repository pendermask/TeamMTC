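; BP_MonsterSpawner is a level actor that places the stage's enemy, or a teleport door when the stage has none mapped.
; On BeginPlay it looks up the level name's suffix after the underscore in SpawnMonsterAndMagician to set the MonsterOrMagician child actor class.
; For a mapped enemy, it registers that component as BP_JYPGMB's CurrentEnemy.
; Unconnected logic for random picks from a per-level index list remains unused.
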(event `self.ReceiveBeginPlay`
  (bind _monsterormagician (`self.MonsterOrMagician`))
  (bind _returnvalue (`GameplayStatics.GetCurrentLevelName` true))
  (bind (_value _returnvalue_2) (`BlueprintMapLibrary.Map_Find` (`self.spawnMonsterAndMagician`) (`.RightS` (`KismetStringLibrary.Split` _returnvalue "_"))))
  (if _returnvalue_2
    (`ChildActorComponent.SetChildActorClass` _monsterormagician _value)
    (bind _asbp_jypgmb (cast `/Game/JYP/Blueprints/BP_JYPGMB` (`GameplayStatics.GetGameMode`)))
    (set `/Game/JYP/Blueprints/BP_JYPGMB.currentEnemy` (`self.MonsterOrMagician`) _asbp_jypgmb)
    (else
      (`ChildActorComponent.SetChildActorClass` _monsterormagician "/Game/JYP/Blueprints/BP_TeleportDoor.BP_TeleportDoor_C"))))

(fn `UserConstructionScript`)