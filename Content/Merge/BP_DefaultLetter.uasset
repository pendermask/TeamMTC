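; Interactable letter for a hand-tracking player that fades in on BeginPlay and unlocks player progression when clicked.
; An opacity timeline drives the Letterz material, then enables interaction on completion, though the highlight component is already set interactable at start.
; WhenClickLetter hides the letter, disables its interaction, reveals the child actor component and sets player flags allowing next-door presses and card opening.
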(event `self.ReceiveBeginPlay`
  ;[0 0 0 0 25] BeginPlay for Init
  (set `self.bInteract?` false)
  (set `/Game/Merge/BP_DefaultHighlightComp.bInteractable?` true (`self.BP_DefaultHighlightComp`))
  (`self.InitLetterAppearance`)
  (bind _asbp_default_hand_tracking_player (cast `/Game/Merge/BP_DefaultHandTrackingPlayer` (`GameplayStatics.GetPlayerPawn` 0)))
  (set `self.Player` _asbp_default_hand_tracking_player))

(event `InitLetterAppearance`
  ;[0 0 0 0 25] Dice Appearance
  (bind (_direction _diceupdate) (`Timeline|LetterAppearance` :!via `PlayFromStart`)
    (:`Update`
      (`MeshComponent.SetScalarParameterValueOnMaterials` (`self.Letterz`) "Opacity" _diceupdate))
    (:`Finished`
      (set `/Game/Merge/BP_DefaultHighlightComp.bInteractable?` true (`self.BP_DefaultHighlightComp`))
      (set `self.bInteract?` true))))

(event `WhenClickLetter`
  (if (`self.bInteract?`)
    (bind _asbp_default_hand_tracking_player (cast `/Game/Merge/BP_DefaultHandTrackingPlayer` (`GameplayStatics.GetPlayerPawn` 0)))
    (set `/Game/Merge/BP_DefaultHandTrackingPlayer.bPlayerCanPressNextDoor?` true _asbp_default_hand_tracking_player)
    (`SceneComponent.SetVisibility` (`self.Letterz`) false false)
    (set `/Game/Merge/BP_DefaultHighlightComp.bInteractable?` false (`self.BP_DefaultHighlightComp`))
    (set `self.bInteract?` false)
    (set `self.bChildInteract?` true)
    (set `/Game/Merge/BP_DefaultHandTrackingPlayer.bPlayerCanCardOpen?` true (`self.Player`))
    (`SceneComponent.SetVisibility` (`self.ChildActor`) true false)))

(fn `UserConstructionScript`)