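; BP_DefaultFriendshipComp tracks a monster's friendship and feeds it into the game-wide total on GI_DGameInstance, cached at BeginPlay.
; GetFriendship adds a random amount up to the passed maximum to the monster's running value and flags it as gained.
; A separate random roll keys the FriendshipDialogue map; on a match, it sets the output dialogue and adds the monster's whole accumulated value to TotalFriendship.
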(event `self.ReceiveBeginPlay`
  ;[1 1 1] Comment
  (bind _asgi_dgame_instance (cast `/Game/Merge/GI_DGameInstance` (`GameplayStatics.GetGameInstance`)))
  (set `self.GameInstance` _asgi_dgame_instance))

(event `GetFriendship`
  (params (friendship :type Integer))
  (bind _returnvalue (`KismetMathLibrary.RandomIntegerInRange` 0 friendship))
  (bind (_value _returnvalue_2) (`BlueprintMapLibrary.Map_Find` (`self.friendshipDialogue`) _returnvalue))
  ;[1 1 1] Comment
  (set `self.randomFriendship` _returnvalue)
  (set `self.bMonsterGetFriendship?` true)
  (bind _output_get (set `self.eachMonsterFriendshipValue` (+ (`self.eachMonsterFriendshipValue`) (`self.randomFriendship`))))
  (if _returnvalue_2
    (set `self.friendshipDialogueOutput` _value)
    (set `/Game/Merge/GI_DGameInstance.totalFriendship` (+ (`/Game/Merge/GI_DGameInstance.totalFriendship` (`self.GameInstance`)) _output_get) (`self.GameInstance`))))