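; VR player hand Blueprint that uses hand tracking to summon, grab and shoot a Strength card.
; Card events spawn BP_08_Strength above the left palm, make it follow the right palm on Tick while grabbed, then launch it forward and destroy it.
; Boolean flags gate each stage, and the P key saves a right-hand shoot gesture to an asset.
; Two-hand dice events set flags toward an empty DoDice stub.
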(event `self.ReceiveBeginPlay`
  (`HeadMountedDisplayFunctionLibrary.SetTrackingOrigin` "Floor"))

(event `Key|P`
  (params (Key :type "Key Structure"))
  (:`Pressed`
    (`HTHandTrackingGestureComponent.SaveGesture` (`self.HTHandTrackingGesture`) "/Game/HOO/RHG_ShootCard.RHG_ShootCard" "Right" false (-1.0 -1.0 -1.0))
    (`KismetSystemLibrary.PrintString` "Saved")))

(event `CardsOn`
  (bind (_returnvalue_x _returnvalue_y _returnvalue_z) (`KismetMathLibrary.BreakVector` (`HandTrackingFL.GetHandPalmLocation` (`self.LeftHandTracking`))))
  (if (not (`self.CardsOn?`))
    (bind _returnvalue (`|SpawnActorFromClass` "/Game/HOO/BP_08_Strength.BP_08_Strength_C" (`KismetMathLibrary.Conv_VectorToTransform` (`KismetMathLibrary.MakeVector` _returnvalue_x _returnvalue_y (+ _returnvalue_z 10.0))) "Undefined" "OverrideRootScale" null null))
    (set `self.CardsOn?` true)))

(event `self.ReceiveTick`
  (params (DeltaSeconds :type "Float (single-precision)"))
  (bind (_returnvalue_x _returnvalue_y _returnvalue_z) (`KismetMathLibrary.BreakVector` (`HandTrackingFL.GetHandPalmLocation` (`self.RightHandTracking`))))
  (`|ExecutionSequence`
    (:`then_0`
      (if (and (`self.GrabOn?`) (not (`self.ShootCard?`)))
        (`self.K2_SetActorLocation` (stale `CardsOn` _returnvalue) (`KismetMathLibrary.MakeVector` _returnvalue_x _returnvalue_y (+ _returnvalue_z 20.0)) false false)))
    (:`then_1`
      (if true
        _))))

(event `CardsOff`
  (if (`self.CardsOn?`)
    (`self.K2_DestroyActor` (stale `CardsOn` _returnvalue))
    (set `self.CardsOn?` false)))

(event `GrabCard`
  (if (`self.CardsOn?`)
    (set `self.GrabOn?` true)))

(event `GrabCancel`
  (if (`self.GrabOn?`)
    (`self.K2_DestroyActor` (stale `CardsOn` _returnvalue))
    (set `self.CardsOn?` false)))

(event `ShootCard`
  (if (`self.GrabOn?`)
    (set `self.ShootCard?` true)
    (`KismetSystemLibrary.MoveComponentTo` (`Actor.RootComponent` (stale `CardsOn` _returnvalue)) (+ (`self.K2_GetActorLocation` self) (* (`self.GetActorForwardVector` self) 500.0)) (struct) false false 1.0)
    (set `self.GrabOn?` false)
    (set `self.CardsOn?` false)
    (`self.K2_DestroyActor` (stale `CardsOn` _returnvalue))
    (set `self.ShootCard?` false)))

(event `Dice_Left`
  (bind _output_get (set `self.Dice_L` true))
  (if (and _output_get (stale `Dice_Right` _output_get))
    (`self.DoDice`)))

(event `Dice_Right`
  (bind _output_get (set `self.Dice_R` true)))

(event `DoDice`)

(fn `UserConstructionScript`)