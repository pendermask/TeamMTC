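; Hand card spawner that fills four child actor components with random card classes from the CardShuffle array on BeginPlay.
; After each pick it calls RemoveIndex, but the pure Random node re-evaluates, so the removed card can differ from the one placed and duplicates remain possible.
; SpawnHnadCard is empty, and unconnected while-loop logic over the 22 Major Arcana tarot classes never runs.
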(event `self.ReceiveBeginPlay`
  (bind _cardshuffle (`self.CardShuffle`))
  (bind (_outitem _outindex) (`KismetArrayLibrary.Array_Random` _cardshuffle))
  (bind (_outitem_2 _outindex_2) (`KismetArrayLibrary.Array_Random` _cardshuffle))
  (bind (_outitem_3 _outindex_3) (`KismetArrayLibrary.Array_Random` _cardshuffle))
  (bind (_outitem_4 _outindex_4) (`KismetArrayLibrary.Array_Random` _cardshuffle))
  (`ChildActorComponent.SetChildActorClass` (`self.ChildActor1`) _outitem)
  (`KismetArrayLibrary.Array_Remove` _cardshuffle _outindex)
  (`ChildActorComponent.SetChildActorClass` (`self.ChildActor2`) _outitem_2)
  (`KismetArrayLibrary.Array_Remove` _cardshuffle _outindex_2)
  (`ChildActorComponent.SetChildActorClass` (`self.ChildActor3`) _outitem_3)
  (`KismetArrayLibrary.Array_Remove` _cardshuffle _outindex_3)
  (`ChildActorComponent.SetChildActorClass` (`self.ChildActor4`) _outitem_4)
  (`KismetArrayLibrary.Array_Remove` _cardshuffle _outindex_4))

(event `SpawnHnadCard`)

(fn `UserConstructionScript`)