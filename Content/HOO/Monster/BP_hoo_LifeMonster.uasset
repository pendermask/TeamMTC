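; BP_hoo_LifeMonster is a monster that heals itself during turn-based play.
; It caches the player character as BP_JYPTestPlayer on BeginPlay.
; When OnMyturn fires and the player's turn flag is off, it heals a small random amount through its health component, then waits and prints the heal and current health.
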(event `self.ReceiveBeginPlay`
  (bind _asbp_jyptest_player (cast `/Game/JYP/Blueprints/BP_JYPTestPlayer` (`GameplayStatics.GetPlayerCharacter` 0)))
  (set `self.Player` _asbp_jyptest_player))

(event `self.OnMyturn`
  (bind _bp_healthcomp (`self.BP_HealthComp`))
  (if (not (`/Game/JYP/Blueprints/BP_JYPTestPlayer.bPlayerTurn?` (`self.Player`)))
    (bind _output_get (set `self.heal` (`KismetMathLibrary.RandomIntegerInRange` 1 3)))
    (`/Game/JYP/Blueprints/BP_HealthComp.Healing` _bp_healthcomp _output_get)
    (`KismetSystemLibrary.Delay` 5.0)
    (`KismetSystemLibrary.PrintString` (`KismetStringLibrary.Concat_StrStr` "current heal : " (`KismetStringLibrary.Conv_IntToString` _output_get) " \ncurrent health" (`KismetStringLibrary.Conv_IntToString` (`/Game/JYP/Blueprints/BP_HealthComp.currenthealth` _bp_healthcomp))))))

(fn `UserConstructionScript`)