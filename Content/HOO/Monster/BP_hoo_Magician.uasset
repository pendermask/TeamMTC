(event `self.ReceiveBeginPlay`)

(event `startDialogue`)

(fn `UserConstructionScript`)