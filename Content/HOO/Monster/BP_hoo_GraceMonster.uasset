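; BP_hoo_GraceMonster is a monster for a turn-based encounter that takes its turn by building friendship instead of attacking.
; On BeginPlay it caches the test player and the game mode.
; OnMyturn, only when it is not the player's turn, adds a small random amount to FriendshipGrace, prints it, waits, then hands the turn back through the game mode's PlayerTurn.
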(event `self.ReceiveBeginPlay`
  (bind _asbp_jyptest_player (cast `/Game/JYP/Blueprints/BP_JYPTestPlayer` (`GameplayStatics.GetPlayerCharacter` 0)))
  (set `self.Player` _asbp_jyptest_player)
  (bind _asbp_jypgmb (cast `/Game/JYP/Blueprints/BP_JYPGMB` (`GameplayStatics.GetGameMode`)))
  (set `self.JYPGMB` _asbp_jypgmb))

(event `self.OnMyturn`
  (if (not (`/Game/JYP/Blueprints/BP_JYPTestPlayer.bPlayerTurn?` (`self.Player`)))
    (bind _output_get (set `self.friendship_Grace` (+ (`KismetMathLibrary.RandomIntegerInRange` 1 3) (`self.friendship_Grace`))))
    (`KismetSystemLibrary.PrintString` (`KismetStringLibrary.Concat_StrStr` "My friendship is " (`KismetStringLibrary.Conv_IntToString` _output_get)))
    (`KismetSystemLibrary.Delay` 5.0)
    (`KismetSystemLibrary.PrintString` "Player Turn !")
    (`/Game/JYP/Blueprints/BP_JYPGMB.PlayerTurn` (`self.JYPGMB`))))

(fn `UserConstructionScript`)