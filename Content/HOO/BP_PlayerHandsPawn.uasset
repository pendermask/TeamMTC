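; VR player pawn with hand tracking that spawns a Strength card (BP_08Strength) at the left palm and lets the right hand carry it.
; CardsOn spawns the card once flagged off, then GrabCard and LooseCard toggle carrying.
; Tick aligns the card's rotation to the Box component with a yaw offset and, while grabbed, moves it to the right palm.
; Pressing P saves the right-hand grab gesture to its asset.
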(event `self.ReceiveBeginPlay`
  (`HeadMountedDisplayFunctionLibrary.SetTrackingOrigin` "Floor"))

(event `Key|P`
  (params (Key :type "Key Structure"))
  (:`Pressed`
    (bind _returnvalue (`HTHandTrackingGestureComponent.SaveGesture` (`self.HTHandTrackingGesture`) "/Game/HOO/HG_RightHandGrabCard.HG_RightHandGrabCard" "Right" false (-1.0 -1.0 -1.0)))
    (`KismetSystemLibrary.PrintString` (`KismetStringLibrary.Conv_BoolToString` _returnvalue))))

(event `CardsOn`
  (if (not (`self.CardsOnHand?`))
    (bind _returnvalue (`|SpawnActorFromClass` "/Game/HOO/BP_08Strength.BP_08Strength_C" (`KismetMathLibrary.Conv_VectorToTransform` (`HandTrackingFL.GetHandPalmLocation` (`self.LeftHand`))) "Undefined" "OverrideRootScale" null null))
    (`/Engine/EditorBlueprintResources/StandardMacros.DoOnce` false
      (:`Completed`
        (set `self.CardsOnHand?` true)))))

(event `self.ReceiveTick`
  (params (DeltaSeconds :type "Float (single-precision)"))
  (bind (_returnvalue_roll _returnvalue_pitch _returnvalue_yaw) (`KismetMathLibrary.BreakRotator` (`SceneComponent.K2_GetComponentRotation` (`self.Box`))))
  (`|ExecutionSequence`
    (:`then_0`
      (if (`self.CardsOnHand?`)
        (`self.K2_SetActorRotation` (stale `CardsOn` _returnvalue) (`KismetMathLibrary.MakeRotator` _returnvalue_roll _returnvalue_pitch (+ _returnvalue_yaw 90.0)) false)))
    (:`then_1`
      (if (`self.GrabCard?`)
        (`self.K2_SetActorLocation` (stale `CardsOn` _returnvalue) (`HandTrackingFL.GetHandPalmLocation` (`self.RightHand`)) false false)))))

(event `GrabCard`
  (if (`self.CardsOnHand?`)
    (set `self.GrabCard?` true)))

(event `LooseCard`
  (set `self.GrabCard?` false))

(fn `UserConstructionScript`)